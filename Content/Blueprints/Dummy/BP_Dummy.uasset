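; Dummy character that reacts to hits and can be backstabbed by BP_Maris.
; A collision overlap with Maris toggles the backstab prompt widget, and any damage plays a montage and launches the dummy along the damage causer's facing.
; Backstab returns a position and rotation for the attacker and triggers a delayed death montage, then DeadSettings disables collision, hides the prompt, starts delayed ragdoll and sets a life span.
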(event `Ragdoll`
  ; Ragdoll
  (`KismetSystemLibrary.Delay` 2.5)
  (`PrimitiveComponent.SetSimulatePhysics` (`self.Mesh`) true))

(event `self.BackStabCollision.OnComponentBeginOverlap`
  (params (OverlappedComponent :type "PrimitiveComponent Object Reference") (OtherActor :type "Actor Object Reference") (OtherComp :type "PrimitiveComponent Object Reference") (OtherBodyIndex :type Integer) (bFromSweep :type Boolean) (SweepResult :type "HitResult Structure (by ref)"))
  ; BackstabVisibility when it is possible
  (if (`GameplayStatics.ObjectIsA` OtherActor "/Game/Blueprints/Maris/BP_Maris.BP_Maris_C")
    (`SceneComponent.SetVisibility` (`self.BackstabWidget`) true false)
    (else
      (`SceneComponent.SetVisibility` (`self.BackstabWidget`) false false :!label _label))))

(event `self.BackStabCollision.OnComponentEndOverlap`
  (params (OverlappedComponent :type "PrimitiveComponent Object Reference") (OtherActor :type "Actor Object Reference") (OtherComp :type "PrimitiveComponent Object Reference") (OtherBodyIndex :type Integer))
  ; BackstabVisibility when it is possible
  (if (`GameplayStatics.ObjectIsA` OtherActor "/Game/Blueprints/Maris/BP_Maris.BP_Maris_C")
    (goto _label)))

(event `SetLifeSpanAfterDied`
  ;[0.15 0.02805 0.02655 0.5] Turn off Widget and set Life Span after died
  (`SceneComponent.SetVisibility` (`self.BackstabWidget`) false false)
  (`self.SetLifeSpan` 600.0))

(event `DieAnimation`
  ; Play dead animation with delay
  (`KismetSystemLibrary.Delay` (`self.BackstabDieAnimationDelay`))
  (`self.PlayAnimMontage` "/Game/Animations/Maris/BackStab/BackStab_vic_UE_Montage.BackStab_vic_UE_Montage")
  (`self.DeadSettings`))

(event `self.ReceiveAnyDamage`
  (params (Damage :type "Float (single-precision)") (DamageType :type "DamageType Object Reference") (InstigatedBy :type "Controller Object Reference") (DamageCauser :type "Actor Object Reference"))
  (bind _hitreactions (`self.HitReactions`))
  (`self.PlayAnimMontage` (`|GetArrayItem` _hitreactions (`KismetMathLibrary.RandomIntegerInRange` 0 (- (`KismetArrayLibrary.Array_Length` _hitreactions) 1))))
  (`self.LaunchCharacter` (* (`KismetMathLibrary.GetForwardVector` (`self.K2_GetActorRotation` DamageCauser)) (`self.HitBackSlip`))))

(fn `Backstab`
  (returns (BackStabberLoc :type "Vector Structure") (BackStabberRot :type "Rotator Structure"))
  (`self.DieAnimation`)
  (return (`SceneComponent.K2_GetComponentLocation` (`self.BackStabRef`)) (`self.K2_GetActorRotation`)))

(fn `DeadSettings`
  (`self.Ragdoll`)
  (`PrimitiveComponent.SetCollisionEnabled` (`self.CapsuleComponent`) "NoCollision")
  (`PrimitiveComponent.SetCollisionEnabled` (`self.BackStabCollision`) "NoCollision")
  (`self.SetLifeSpanAfterDied`))

(fn `UserConstructionScript`)