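; Base AI controller for enemies that runs the possessed BP_EnemyBase's behavior tree and drives its Blackboard state: Passive, Investigating, Combat, Seeking, Frozen or Dead.
; Sight and damage from other teams trigger combat, while hearing triggers investigation.
; Losing sight of the target starts a delayed switch to seeking its location.
; A looping timer polls for forgotten seen actors, returning to Passive when the target is forgotten.
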(event `self.ReceivePossess`
  (params (PossessedPawn :type "Pawn Object Reference"))
  (bind _blackboard (`self.Blackboard`))
  (bind _output_get (set `self.Possessed Pawn` PossessedPawn))
  ;[0.04801 0.05208 0.05083] Run Selected Behaviour Tree
  (bind _asbp_enemy_base (cast `/Game/Blueprints/Enemies/BP_EnemyBase` _output_get))
  (bind _behaviourtree (`/Game/Blueprints/Enemies/BP_EnemyBase.BehaviourTree` _asbp_enemy_base)
    (:`then`
      (`self.RunBehaviorTree` _behaviourtree)
      ;[0.04801 0.05208 0.05083] Set Default State
      (`self.SetStateAsPassive`)
      (bind (_attackradius _defendradius) (message `/Game/Blueprints/AI/BPI_EnemyAI.AI_GetIdealRange` (`self.Possessed Pawn`)))
      (`BlackboardComponent.SetValueAsFloat` _blackboard (`self.AttackRadiusKeyName`) _attackradius)
      (`BlackboardComponent.SetValueAsFloat` _blackboard (`self.DefendRadiusKeyName`) _defendradius)
      ; Check Forgetten Actors Loop
      (bind _returnvalue (`KismetSystemLibrary.K2_SetTimerDelegate` (`|CreateDelegate` :!event `CheckForgettenSeen`) 0.01 true))
      (set `self.CheckForgottenActorsTimer` _returnvalue))
    (:`else`)))

(event `self.ReceiveUnPossess`
  (params (UnpossessedPawn :type "Pawn Object Reference"))
  (`KismetSystemLibrary.K2_ClearAndInvalidateTimerHandle` (`self.CheckForgottenActorsTimer`)))

(event `StartSeeking`
  (`self.SetStateAsSeeking` (`self.K2_GetActorLocation` (`self.Attack Target`))))

(event `self.AIPerception.OnPerceptionUpdated`
  (params (UpdatedActors :type "Array of Actor Object Reference (by ref)"))
  ;[0.5938 0.5153 0 0.5] Perception Process
  (for _array_element UpdatedActors
    (`|ExecutionSequence`
      (:`then_0`
        (bind _sensed (`self.CanSenseActor` _array_element "NewEnumerator1"))
        (if _sensed
          (`self.HandleSensedSight` _array_element)
          (else
            (`self.HandleLostSight` _array_element))))
      (:`then_1`
        (bind (_sensed_2 _stimulus) (`self.CanSenseActor` _array_element "NewEnumerator2"))
        (if _sensed_2
          (`self.HandleSensedHearing` (`.StimulusLocation` (break `AIStimulus` _stimulus)))))
      (:`then_2`
        (bind _sensed_3 (`self.CanSenseActor` _array_element "NewEnumerator3"))
        (if _sensed_3
          (`self.HandleSensedDamage` _array_element))))))

(event `/Game/Blueprints/AI/BPI_AIController.SetPassive`
  ;[1 0.1067 0] States Interface
  (`self.SetStateAsPassive`))

(event `CheckForgettenSeen`
  ;[0.04801 0.05208 0.05083] Forget Actor
  (if (!= (`KismetArrayLibrary.Array_Length` (`self.KnownSeenActors`)) (`KismetArrayLibrary.Array_Length` (`AIPerceptionComponent.GetKnownPerceivedActors` (`self.AIPerception`) "/Script/AIModule.AISense_Sight")))
    (for _array_element (`self.KnownSeenActors`)
      (if (== (`KismetArrayLibrary.Array_Find` (`AIPerceptionComponent.GetKnownPerceivedActors` (`self.AIPerception`) "/Script/AIModule.AISense_Sight") _array_element) -1)
        (`self.HandleForgotActor` _array_element)))))

(event `/Game/Blueprints/AI/BPI_AIController.SetCombat`
  (params (AttackTarget :type "Actor Object Reference") (UseLastKnownTarget :type Boolean))
  ;[1 0.1067 0] States Interface
  (`self.SetStateAsCombat` AttackTarget UseLastKnownTarget))

(event `/Game/Blueprints/AI/BPI_AIController.SetFrozen`
  ;[1 0.1067 0] States Interface
  (`self.SetStateAsFrozen`))

(event `/Game/Blueprints/AI/BPI_AIController.SetInvestigating`
  (params (Location :type "Vector Structure"))
  ;[1 0.1067 0] States Interface
  (`self.SetStateAsInvenstigating` Location))

(event `/Game/Blueprints/AI/BPI_AIController.SetDead`
  ;[1 0.1067 0] States Interface
  (`self.SetStateAsDead`))

(fn `CanSenseActor`
  (params (Actor :type "Actor Object Reference") (Sense :type "/Game/Blueprints/AI/Enums/E_AISenses Enum" :default "NewEnumerator0"))
  (returns (Sensed :type Boolean) (Stimulus :type "AIStimulus Structure"))
  (bind _info (`AIPerceptionComponent.GetActorsPerception` (`self.AIPerception`) Actor))
  (for _array_element (`.LastSensedStimuli` (break `ActorPerceptionBlueprintInfo` _info))
    (bind _returnvalue (`AIPerceptionSystem.GetSenseClassForStimulus` _array_element))
    (if (== _returnvalue (select `/Game/Blueprints/AI/Enums/E_AISenses` Sense :`NewEnumerator1` "/Script/AIModule.AISense_Sight" :`NewEnumerator2` "/Script/AIModule.AISense_Hearing" :`NewEnumerator3` "/Script/AIModule.AISense_Damage" :!type "Object Class Reference"))
      (return (`.bSuccessfullySensed` (break `AIStimulus` _array_element)) _array_element))))

(fn `GetAttackTarget`
  (returns (AttackTarget :type "Actor Object Reference"))
  (return (`self.Attack Target`)))

(fn `GetCurrentState`
  (returns (CurrentState :type "/Game/Blueprints/AI/Enums/E_AIStates Enum"))
  (return (cast `/Game/Blueprints/AI/Enums/E_AIStates` (`BlackboardComponent.GetValueAsEnum` (`self.Blackboard`) (`self.StateEnumKeyName`)))))

(fn `HandleForgotActor`
  (params (Actor :type "Actor Object Reference"))
  (`KismetArrayLibrary.Array_RemoveItem` (`self.KnownSeenActors`))
  (if (== Actor (`self.Attack Target`))
    (`self.SetStateAsPassive`)))

(fn `HandleLostSight`
  (params (AttackTarget :type "Actor Object Reference"))
  (if (== AttackTarget (`self.Attack Target`))
    (bind _currentstate (`self.GetCurrentState`))
    (switch `/Game/Blueprints/AI/Enums/E_AIStates` _currentstate
      (:`NewEnumerator1`
        _)
      (:`NewEnumerator2`
        _)
      (:`NewEnumerator4`
        _))
    (`KismetSystemLibrary.K2_ClearAndInvalidateTimerHandle` (`self.StartSeekingTimer`))
    (bind _returnvalue (`KismetSystemLibrary.K2_SetTimerDelegate` (`|CreateDelegate` :!event `StartSeeking`) (`self.StartSeekingDelay`)))
    (set `self.StartSeekingTimer` _returnvalue)))

(fn `HandleSensedDamage`
  (params (`Damage Causer` :type "Actor Object Reference"))
  (bind _onsameteam (`self.OnSameTeam` `Damage Causer`))
  (if (not _onsameteam)
    (bind _currentstate (`self.GetCurrentState`))
    (switch `/Game/Blueprints/AI/Enums/E_AIStates` _currentstate
      (:`NewEnumerator0`
        _)
      (:`NewEnumerator4`
        _)
      (:`NewEnumerator6`
        _))
    (`self.SetStateAsCombat` (`local.Damage Causer`))))

(fn `HandleSensedHearing`
  (params (Location :type "Vector Structure"))
  (bind _currentstate (`self.GetCurrentState`))
  (switch `/Game/Blueprints/AI/Enums/E_AIStates` _currentstate
    (:`NewEnumerator0`
      _)
    (:`NewEnumerator4`
      _)
    (:`NewEnumerator6`
      _))
  (`self.SetStateAsInvenstigating` Location))

(fn `HandleSensedSight`
  (params (AttackTarget :type "Actor Object Reference"))
  (`KismetArrayLibrary.Array_AddUnique` (`self.KnownSeenActors`) AttackTarget)
  (bind _currentstate (`self.GetCurrentState`))
  (bind _onsameteam (`self.OnSameTeam` AttackTarget))
  (if (not _onsameteam)
    (switch `/Game/Blueprints/AI/Enums/E_AIStates` _currentstate
      (:`NewEnumerator0`
        (`self.SetStateAsCombat` (`local.AttackTarget`) :!label _label)
        (return))
      (:`NewEnumerator1`
        ; Don't seek if seen again
        (if (== AttackTarget (`self.Attack Target`))
          (`KismetSystemLibrary.K2_ClearAndInvalidateTimerHandle` (`self.StartSeekingTimer`))))
      (:`NewEnumerator4`
        (goto _label))
      (:`NewEnumerator6`
        (goto _label)))))

(fn `OnSameTeam`
  (params (Actor :type "Actor Object Reference"))
  (returns (OnSameTeam :type Boolean))
  (bind _teamnumber (message `/Game/Blueprints/DamageSystem/BPI_StatManagement.GetTeamNumber` Actor))
  (bind _teamnumber_2 (message `/Game/Blueprints/DamageSystem/BPI_StatManagement.GetTeamNumber` (`self.K2_GetPawn`)))
  (return (== _teamnumber_2 _teamnumber)))

(fn `SetStateAsCombat`
  (params (AttackTarget :type "Actor Object Reference") (UseLastKnownTarget :type Boolean))
  (locals (NewAttackTarget :type "Actor Object Reference"))
  (bind _output_get (set `local.NewAttackTarget` (select `bool` (and UseLastKnownTarget (`KismetSystemLibrary.IsValid` (`self.Attack Target`))) :`false` AttackTarget :`true` (`self.Attack Target`))))
  (`/Engine/EditorBlueprintResources/StandardMacros.IsValid` _output_get
    (:`Is Valid`
      (bind (_maxhealth _currenthealth _isdead_) (message `/Game/Blueprints/DamageSystem/BPI_StatManagement.GetHealthValues` _output_get))
      (if (not _isdead_)
        (`BlackboardComponent.SetValueAsObject` (`self.Blackboard`) (`self.AttackTargetKeyName`) _output_get)
        (`BlackboardComponent.SetValueAsEnum` (`self.Blackboard`) (`self.StateEnumKeyName`) (enumliteral `/Game/Blueprints/AI/Enums/E_AIStates` "NewEnumerator1"))
        (set `self.Attack Target` _output_get)
        (else
          (`self.SetStateAsPassive` :!label _label))))
    (:`Is Not Valid`
      (goto _label))))

(fn `SetStateAsDead`
  (`BlackboardComponent.SetValueAsEnum` (`self.Blackboard`) (`self.StateEnumKeyName`) (enumliteral `/Game/Blueprints/AI/Enums/E_AIStates` "NewEnumerator5")))

(fn `SetStateAsFrozen`
  (`BlackboardComponent.SetValueAsEnum` (`self.Blackboard`) (`self.StateEnumKeyName`) (enumliteral `/Game/Blueprints/AI/Enums/E_AIStates` "NewEnumerator2")))

(fn `SetStateAsInvenstigating`
  (params (Location :type "Vector Structure"))
  (bind _blackboard (`self.Blackboard`))
  (`BlackboardComponent.SetValueAsEnum` _blackboard (`self.StateEnumKeyName`) (enumliteral `/Game/Blueprints/AI/Enums/E_AIStates` "NewEnumerator4"))
  (`BlackboardComponent.SetValueAsVector` _blackboard (`self.PointOfInterestKeyName`) (`local.Location`)))

(fn `SetStateAsPassive`
  (`BlackboardComponent.SetValueAsEnum` (`self.Blackboard`) (`self.StateEnumKeyName`) (enumliteral `/Game/Blueprints/AI/Enums/E_AIStates` "NewEnumerator0")))

(fn `SetStateAsSeeking`
  (params (Location :type "Vector Structure"))
  (bind _blackboard (`self.Blackboard`))
  (`BlackboardComponent.SetValueAsEnum` _blackboard (`self.StateEnumKeyName`) (enumliteral `/Game/Blueprints/AI/Enums/E_AIStates` "NewEnumerator6"))
  (`BlackboardComponent.SetValueAsVector` _blackboard (`self.PointOfInterestKeyName`) Location))

(fn `UserConstructionScript`)