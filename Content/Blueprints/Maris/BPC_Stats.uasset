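; BPC_Stats is a stats component that tracks health and stamina, handles damage, healing and death, and fills progress bars for both values.
; TakeDamage uses the CanBeDamaged macro to route hits to block, damage or no damage based on invincibility, death and blocking.
; It fires dispatchers for blocks, death and interruptible damage responses.
; Stamina functions clamp depletion and regeneration, flag exhaustion, and spend guard stamina only when some would remain.
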(fn `CalculateHealthBar`
  (params (HealthBar :type "ProgressBar Object Reference"))
  (`ProgressBar.SetPercent` HealthBar (/ (`self.CurrentHealth`) (`self.MaxHealth`)))
  (return))

(fn `CalculateStaminaBar`
  (params (StaminaBar :type "ProgressBar Object Reference"))
  (`ProgressBar.SetPercent` StaminaBar (/ (`self.CurrentStamina`) (`self.MaxStamina`))))

(fn `Heal`
  (params (RegenerationAmount :type "Float (double-precision)"))
  (returns (NewHealth :type "Float (double-precision)"))
  (if (not (`self.IsDead`))
    (bind _output_get (set `self.CurrentHealth` (`KismetMathLibrary.FClamp` (+ (`local.RegenerationAmount`) (`self.CurrentHealth`)) 0.0 (`self.MaxHealth`))))
    (return _output_get)))

(fn `IncreaseMaxHealth`
  (params (`Health Increment` :type "Float (double-precision)"))
  (set `self.MaxHealth` (+ `Health Increment` (`self.MaxHealth`))))

(fn `StaminaDeplete`
  (params (StaminaDepValue :type "Float (double-precision)"))
  (returns (IsStaminaDepleted :type Boolean))
  (bind _returnvalue (`KismetMathLibrary.FClamp` (- (`self.CurrentStamina`) (`local.StaminaDepValue`)) 0.0 (`self.MaxStamina`)))
  (set `self.CurrentStamina` _returnvalue)
  (if (<= _returnvalue 0.0)
    (bind _output_get (set `self.IsStaminaDepleted?` true))
    (return _output_get)
    (else
      (bind _output_get_2 (set `self.IsStaminaDepleted?` false))
      (return _output_get_2))))

(fn `StaminaGuardDeplete`
  (params (Damage :type "Float (double-precision)"))
  (returns (Blocked :type Boolean))
  (if (> (- (`self.CurrentStamina`) (`local.Damage`)) 0.0)
    (set `self.CurrentStamina` (- (`self.CurrentStamina`) (`local.Damage`)))
    (return true)
    (else
      (return false))))

(fn `StaminaRegeneration`
  (params (StaminaRegenValue :type "Float (double-precision)"))
  (bind _output_get (set `self.CurrentStamina` (`KismetMathLibrary.FClamp` (+ StaminaRegenValue (`self.CurrentStamina`)) 0.0 (`self.MaxStamina`))))
  (set `self.IsStaminaDepleted?` (not (> _output_get 0.0))))

(fn `TakeDamage`
  (params (DamageInfo :type "/Game/DamageSystem/S_DamageInfo Structure") (DamageCauser :type "Actor Object Reference"))
  (returns (WasDamaged :type Boolean))
  (bind (_amount _damagetype _damageresponse _shoulddamageinvincible _canbeblocked _canbeparried _shouldforceinterrupt) (break `/Game/DamageSystem/S_DamageInfo` DamageInfo))
  (`self.CanBeDamaged` _shoulddamageinvincible _canbeblocked
    (:`BlockDamage`
      (`self.OnBlocked` _canbeparried _amount)
      (return false))
    (:`DoDamage`
      (bind _output_get (set `self.CurrentHealth` (- (`self.CurrentHealth`) _amount)))
      (if (<= _output_get 0.0)
        (set `self.IsDead` true)
        (`self.OnDeath` DamageCauser)
        (return true)
        (elif (or _shouldforceinterrupt (`self.IsInterruptible`))
          (`self.OnDamageResponse` _damageresponse DamageCauser)
          (return true))))
    (:`NoDamage`
      (return false))))