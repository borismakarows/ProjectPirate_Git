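; Attack component for BP_Maris that runs a three-step sword combo and applies its hit damage.
; IA_Attack plays the montage for the current ComboIndex, while AttackCombo either continues on SaveAttack or resets the chain.
; StartWeaponTrace loops a timer-driven sphere trace between two weapon points, skipped during critical attacks.
; Living BPI_StatManagement targets receive damage and an AI damage report, with camera shake and a short re-hit lockout on success.
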(event `self.ReceiveBeginPlay`
  (`self.StoreKeyVariables`))

(event `EnhancedInput|/Game/Input/Actions/IA_Attack`
  (params (ActionValue :type Boolean) (ElapsedSeconds :type "Float (double-precision)") (TriggeredSeconds :type "Float (double-precision)") (InputAction :type "InputAction Object Reference" :default "/Game/Input/Actions/IA_Attack.IA_Attack"))
  ;[0.15 0 0.003356 0.5] Combo Attack
  ;; Input
  (:`Started`
    (if (`self.CanAttack`)
      (`self.Attack`))))

(event `Attack1`
  ;[0.15 0 0.003356 0.5] Combo Attack
  ;; Attack1
  (`/Engine/EditorBlueprintResources/StandardMacros.DoOnce` false :!label _label
    (:`Completed`
      (`KismetSystemLibrary.Delay` 0.1)
      (`|PlayMontage` (`self.CharacterSKM`) "/Game/Animation/Maris/Attack/Attack1_Montage.Attack1_Montage" 1.1
        (:`then`
          (set `self.ComboIndex` 1)
          (goto _label :!via `Reset`))))))

(event `Attack`
  ;[0.15 0 0.003356 0.5] Combo Attack
  ;; Attack
  (if (`self.SaveAttack`)
    (set `self.SaveAttack` true)
    (else
      (set `self.IsAttacking` true)
      (switch `int` (`self.ComboIndex`) :!label _label_2
        (:`0`
          (`self.Attack1`))
        (:`1`
          (`self.Attack2`))
        (:`2`
          (`self.Attack3`))))))

(event `Attack2`
  ;[0.15 0 0.003356 0.5] Combo Attack
  ;; Attack 2
  (`/Engine/EditorBlueprintResources/StandardMacros.DoOnce` false :!label _label_3
    (:`Completed`
      (`KismetSystemLibrary.Delay` (`self.ComboDelay`))
      (`|PlayMontage` (`self.CharacterSKM`) "/Game/Animation/Maris/Attack/Attack2_Montage.Attack2_Montage" 1.1
        (:`then`
          (set `self.ComboIndex` 2)
          (goto _label_3 :!via `Reset`))))))

(event `AttackCombo`
  ;[0.15 0 0.003356 0.5] Combo Attack
  ;; ContinueAttackCombo
  (if (`self.SaveAttack`)
    (set `self.SaveAttack` false)
    (goto _label_2)
    (else
      (`self.StopAttackCombo`))))

(event `Attack3`
  ;[0.15 0 0.003356 0.5] Combo Attack
  ;; Attack 3
  (`/Engine/EditorBlueprintResources/StandardMacros.DoOnce` false :!label _label_4
    (:`Completed`
      (`KismetSystemLibrary.Delay` (`self.ComboDelay`))
      (`|PlayMontage` (`self.CharacterSKM`) "/Game/Animation/Maris/Attack/Attack3_Montage.Attack3_Montage" 0.8
        (:`then`
          (set `self.ComboIndex` 3)
          (goto _label_4 :!via `Reset`))))))

(event `StopAttackCombo`
  ;[0.15 0 0.003356 0.5] Combo Attack
  ;; StopAttackCombo
  (set `self.IsAttacking` false)
  (set `self.ComboIndex` 0))

(event `StartWeaponTrace`
  ;[1 0.4181 0 0.5] Sword Trace
  (bind _returnvalue (`KismetSystemLibrary.K2_SetTimerDelegate` (delegate `WeaponTraceLoop`) 0.001 true))
  (set `self.SwordTraceTimer` _returnvalue))

(event `WeaponTraceLoop`
  (bind _bp_maris (`self.BP_Maris`))
  ;[1 0.4181 0 0.5] Sword Trace
  (bind _bp_maris_2 (`self.BP_Maris`)
    (:`then`
      (if (not (`/Game/Blueprints/Maris/BP_Maris.IsCriticAttacking` _bp_maris_2))
        (bind (_outhit _returnvalue) (`KismetSystemLibrary.SphereTraceSingle` (`SceneComponent.K2_GetComponentLocation` (`/Game/Blueprints/Maris/BP_Maris.WeaponTopPoint` (`self.BP_Maris`))) (`SceneComponent.K2_GetComponentLocation` (`/Game/Blueprints/Maris/BP_Maris.WeaponEndPoint` (`self.BP_Maris`))) 7.0 "TraceTypeQuery4" false (`|MakeArray` (`self.BP_Maris`) :!type "Actor Object Reference") "None" true (struct :`R` 1.0 :`A` 1.0) (struct :`G` 1.0 :`A` 1.0) 2.0))
        (if _returnvalue
          (bind (_bblockinghit _binitialoverlap _time _distance _location _impactpoint _normal _impactnormal _physmat _hitactor) (`GameplayStatics.BreakHitResult` _outhit))
          (if (`KismetSystemLibrary.DoesImplementInterface` _hitactor "/Game/DamageSystem/BPI_StatManagement.BPI_StatManagement_C")
            (bind (_maxhealth _currenthealth _isdead_) (message `/Game/DamageSystem/BPI_StatManagement.GetHealthValues` _hitactor))
            (if (not _isdead_)
              (`/Engine/EditorBlueprintResources/StandardMacros.DoOnce` false :!label _label_5
                (:`Completed`
                  (`AISense_Damage.ReportDamageEvent` _hitactor _bp_maris 0.0 (`Actor.K2_GetActorLocation` _bp_maris))
                  (bind _wasdamaged (message `/Game/DamageSystem/BPI_StatManagement.TakeDamage` _hitactor (make `/Game/DamageSystem/S_DamageInfo` 20.0 "NewEnumerator1" "NewEnumerator1")))
                  (if _wasdamaged
                    (`GameplayStatics.PlayWorldCameraShake` "/Game/Blueprints/Maris/BP_EnemyHitCameraShake.BP_EnemyHitCameraShake_C" _location 0.0 2000.0)
                    (`KismetSystemLibrary.Delay` 0.6)
                    (goto _label_5 :!via `Reset`)))))))))
    (:`else`)))

(event `StopWeaponTrace`
  ;[1 0.4181 0 0.5] Sword Trace
  (`KismetSystemLibrary.K2_ClearAndInvalidateTimerHandle` (`self.SwordTraceTimer`)))

(fn `StoreKeyVariables`
  (bind _asbp_maris (cast `/Game/Blueprints/Maris/BP_Maris` (`self.GetOwner`)))
  (bind _output_get (set `self.BP_Maris` _asbp_maris))
  (set `self.CharacterSKM` (`Character.Mesh` _output_get)))