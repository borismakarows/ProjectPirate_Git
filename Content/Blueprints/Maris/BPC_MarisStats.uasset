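; Stats component for the BP_Maris character that tracks health and stamina and updates their HUD bars.
; Functions damage, regenerate or deplete each stat within its limits, or raise max health, then set the matching bar's percent on the owner's HudWidget.
; Guard damage drains stamina, but when stamina cannot cover the hit, the full damage goes to health and stamina stays unchanged.
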(event `self.ReceiveBeginPlay`
  (bind _asbp_maris (cast `/Game/Blueprints/Maris/BP_Maris` (`self.GetOwner`)))
  (set `self.Character` _asbp_maris))

(fn `CalculateHealthBar`
  (`ProgressBar.SetPercent` (`/Game/UI/WBP_HUD.HealthBar` (`/Game/Blueprints/Maris/BP_Maris.HudWidget` (`self.Character`))) (/ (`self.CurrentHealth`) (`self.MaxHealth`)))
  (return))

(fn `CalculateStaminaBar`
  (`ProgressBar.SetPercent` (`/Game/UI/WBP_HUD.StaminaBar` (`/Game/Blueprints/Maris/BP_Maris.HudWidget` (`self.Character`))) (/ (`self.CurrentStamina`) (`self.MaxStamina`))))

(fn `GetDamageHealth`
  (params (Damage :type "Float (double-precision)"))
  (bind _returnvalue (- (`self.CurrentHealth`) (`local.Damage`)))
  (if (<= _returnvalue 0.0)
    (set `self.CurrentHealth` 0.0)
    (else
      (set `self.CurrentHealth` _returnvalue)))
  (`self.CalculateHealthBar`))

(fn `HealthRegeneration`
  (params (RegenerationValue :type "Float (double-precision)"))
  (bind _maxhealth (`self.MaxHealth`))
  (bind _returnvalue (+ RegenerationValue (`self.CurrentHealth`)))
  (if (< _returnvalue _maxhealth)
    (set `self.CurrentHealth` _returnvalue)
    (else
      (set `self.CurrentHealth` _maxhealth)))
  (`self.CalculateHealthBar`))

(fn `IncreaseMaxHealth`
  (params (`Health Increment` :type "Float (double-precision)"))
  (set `self.MaxHealth` (+ `Health Increment` (`self.MaxHealth`)))
  (`self.CalculateHealthBar`))

(fn `StaminaDeplete`
  (params (StaminaDepValue :type "Float (double-precision)"))
  (returns (HasStamina :type Boolean))
  (bind _returnvalue (- (`self.CurrentStamina`) (`local.StaminaDepValue`)))
  (bind _returnvalue_2 (<= _returnvalue 0.0))
  (if _returnvalue_2
    (set `self.CurrentStamina` 0.0)
    (else
      (set `self.CurrentStamina` _returnvalue)))
  (`self.CalculateStaminaBar`)
  (return _returnvalue_2))

(fn `StaminaGuardDeplete`
  (params (Damage :type "Float (double-precision)"))
  (if (> (- (`self.CurrentStamina`) (`local.Damage`)) 0.0)
    (set `self.CurrentStamina` (- (`self.CurrentStamina`) (`local.Damage`)))
    (else
      (`self.GetDamageHealth` (`local.Damage`))))
  (`self.CalculateStaminaBar`))

(fn `StaminaRegeneration`
  (params (StaminaRegenValue :type "Float (double-precision)"))
  (bind _maxstamina (`self.MaxStamina`))
  (bind _returnvalue (+ StaminaRegenValue (`self.CurrentStamina`)))
  (if (>= _returnvalue _maxstamina)
    (set `self.CurrentStamina` _maxstamina)
    (else
      (set `self.CurrentStamina` _returnvalue)))
  (`self.CalculateStaminaBar`))