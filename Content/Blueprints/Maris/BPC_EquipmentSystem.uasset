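; Equipment component for the BP_Maris character that handles item pickup and the inventory screen.
; Interact sphere-traces from the follow camera, adds a hit BP_MasterItem's data to the slot array and destroys the actor.
; The inventory input toggles a lazily created WBP_Inventory fed with the slots and weapon mesh sockets.
; Toggling also switches input mode, cursor, movement, attack, crouch and vault, with an equipment UI capture for the screen.
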(event `self.ReceiveBeginPlay`
  (`self.StoreKeyVariables`))

(event `EnhancedInput|/Game/Input/Actions/IA_Interact`
  (params (ActionValue :type Boolean) (ElapsedSeconds :type "Float (double-precision)") (TriggeredSeconds :type "Float (double-precision)") (InputAction :type "InputAction Object Reference" :default "/Game/Input/Actions/IA_Interact.IA_Interact"))
  (bind _follow_camera (`self.Follow Camera`))
  (bind _returnvalue (`SceneComponent.K2_GetComponentLocation` _follow_camera))
  ;[0.7396 0.04308 0 0.5] Interact
  (:`Started`
    (bind _outhit (`KismetSystemLibrary.SphereTraceSingle` :`Start` _returnvalue :`End` (+ _returnvalue (* (`KismetMathLibrary.GetForwardVector` (`SceneComponent.K2_GetComponentRotation` _follow_camera)) 700.0)) :`Radius` 15.0 :`TraceChannel` "TraceTypeQuery5" :`DrawDebugType` "ForDuration"))
    (bind (_bblockinghit _binitialoverlap _time _distance _location _impactpoint _normal _impactnormal _physmat _hitactor) (`GameplayStatics.BreakHitResult` _outhit))
    (bind _asbp_master_item (cast `/Game/InventorySystem/BP_MasterItem` _hitactor))
    (`self.AddToInventory` (`/Game/InventorySystem/BP_MasterItem.ItemData` _asbp_master_item))
    (`Actor.K2_DestroyActor` _hitactor)))

(event `EnhancedInput|/Game/Input/Actions/IA_Inventory`
  (params (ActionValue :type Boolean) (ElapsedSeconds :type "Float (double-precision)") (TriggeredSeconds :type "Float (double-precision)") (InputAction :type "InputAction Object Reference" :default "/Game/Input/Actions/IA_Inventory.IA_Inventory"))
  (bind _returnvalue (`GameplayStatics.GetPlayerController` 0))
  (bind _bp_maris (`self.BP Maris`))
  (bind _bp_maris_2 (`self.BP Maris`))
  ;[0.07656 0.15 0 0.5] Inventory
  (:`Started`
    (`self.WBP Inventory`
      (:`then`
        (if (`Widget.IsVisible` (`self.WBP Inventory`))
          (`Widget.RemoveFromParent` (`self.WBP Inventory`))
          (`WidgetBlueprintLibrary.SetInputMode_GameOnly` _returnvalue)
          (set `PlayerController.bShowMouseCursor` false _returnvalue)
          (`CharacterMovementComponent.SetMovementMode` (`Character.CharacterMovement` _bp_maris) "MOVE_Walking" 0)
          (set `/Game/Blueprints/Maris/BPC_AttackSystem.CanAttack` true (`/Game/Blueprints/Maris/BP_Maris.BPC_AttackSystem` _bp_maris))
          (set `/Game/Blueprints/Maris/BP_Maris.CanCrouch?` true _bp_maris)
          (set `/Game/Blueprints/Maris/BP_Maris.CanVault?` true _bp_maris)
          (`self.SetActive` (`/Game/Blueprints/Maris/BP_Maris.EquipmentUICapture` _bp_maris) false false)
          (`KismetSystemLibrary.Delay` 0.1)
          (else
            (`UserWidget.AddToViewport` (stale _output_get) 0 :!label _label)
            (`WidgetBlueprintLibrary.SetInputMode_GameAndUIEx` (`GameplayStatics.GetPlayerController` 0) (`self.WBP Inventory`))
            (set `PlayerController.bShowMouseCursor` true (`GameplayStatics.GetPlayerController` 0))
            (`/Game/UI/WBP_Inventory.UpdateInventory` (`self.WBP Inventory`) (`self.S_Slots`))
            (`CharacterMovementComponent.SetMovementMode` (`Character.CharacterMovement` _bp_maris_2) "MOVE_None" 0)
            (set `/Game/Blueprints/Maris/BPC_AttackSystem.CanAttack` false (`/Game/Blueprints/Maris/BP_Maris.BPC_AttackSystem` _bp_maris_2))
            (set `/Game/Blueprints/Maris/BP_Maris.CanCrouch?` false _bp_maris_2)
            (set `/Game/Blueprints/Maris/BP_Maris.CanVault?` false _bp_maris_2)
            (`/Game/UI/WBP_Inventory.GetStaticMeshComponent` (`self.WBP Inventory`) (`/Game/Blueprints/Maris/BP_Maris.SwordMeshSocket` _bp_maris_2) (`/Game/Blueprints/Maris/BP_Maris.GunMeshSocket` _bp_maris_2)))))
      (:`else`
        (`self.SetActive` (`/Game/Blueprints/Maris/BP_Maris.EquipmentUICapture` (`self.BP Maris`)) true false)
        (bind _returnvalue_2 (`|CreateWidget` "/Game/UI/WBP_Inventory.WBP_Inventory_C" null (`self.S_Slots`)))
        (bind _output_get (set `self.WBP Inventory` _returnvalue_2))
        (goto _label)))))

(fn `AddToInventory`
  (params (NewItem :type "/Game/InventorySystem/S_Slots Structure (by ref)"))
  (`KismetArrayLibrary.Array_Add` (`self.S_Slots`) NewItem))

(fn `StoreKeyVariables`
  (bind _asbp_maris (cast `/Game/Blueprints/Maris/BP_Maris` (`self.GetOwner`)))
  (bind _output_get (set `self.BP Maris` _asbp_maris))
  (set `self.Follow Camera` (`/Game/Blueprints/Maris/BP_Maris.FollowCamera` _output_get)))