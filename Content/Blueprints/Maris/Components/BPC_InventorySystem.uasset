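; Inventory component for the Maris character that handles item pickup, note reading, the inventory screen and equipping gear.
; Interact sphere-traces, adding master item data to the slot array and destroying the actor, or opening a note's widget.
; The inventory toggle swaps input mode, locks movement and activates a UI capture and light for character preview.
; The widget's equip event routes items by type to functions setting icons, meshes and ammo or capacity values.
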(event `self.ReceiveBeginPlay`
  (`self.StoreKeyVariables`))

(event `EnhancedInput|/Game/Input/Actions/Menu/IA_Interact`
  (params (ActionValue :type Boolean) (ElapsedSeconds :type "Float (double-precision)") (TriggeredSeconds :type "Float (double-precision)") (InputAction :type "InputAction Object Reference" :default "/Game/Input/Actions/Menu/IA_Interact.IA_Interact"))
  (bind _bp_maris (`self.BP Maris`))
  ;[0.7396 0.04308 0 0.5] Interact
  (:`Started`
    (bind (_outhit _returnvalue) (`KismetSystemLibrary.SphereTraceSingle` (`SceneComponent.K2_GetComponentLocation` (`/Game/Blueprints/Maris/BP_Maris.FollowCamera` _bp_maris)) (+ (`SceneComponent.K2_GetComponentLocation` (`/Game/Blueprints/Maris/BP_Maris.FollowCamera` _bp_maris)) (* (`KismetMathLibrary.GetForwardVector` (`SceneComponent.K2_GetComponentRotation` (`self.Follow Camera`))) 700.0)) 110.0 "TraceTypeQuery4" false (`|MakeArray` (`self.BP Maris`) :!type "Actor Object Reference") "ForDuration" true (struct :`R` 1.0 :`A` 1.0) (struct :`G` 1.0 :`A` 1.0) 2.0))
    (if _returnvalue
      (bind (_bblockinghit _binitialoverlap _time _distance _location _impactpoint _normal _impactnormal _physmat _hitactor) (`GameplayStatics.BreakHitResult` _outhit))
      (bind _asbp_master_item (cast `/Game/Blueprints/InventorySystem/BP_MasterItem` _hitactor)
        (:`then`
          (`self.AddToInventory` (`/Game/Blueprints/InventorySystem/BP_MasterItem.ItemData` _asbp_master_item))
          (`Actor.K2_DestroyActor` _hitactor))
        (:`CastFailed`
          (bind _asbp_master_note (cast `/Game/Blueprints/InventorySystem/Notes/BP_MasterNote` _hitactor))
          (`/Game/Blueprints/InventorySystem/Notes/BP_MasterNote.SetTextAndCreateWidget` _asbp_master_note)
          (`MovementComponent.StopMovementImmediately` (`Character.CharacterMovement` (`self.BP Maris`))))))))

(event `EnhancedInput|/Game/Input/Actions/Menu/IA_Inventory`
  (params (ActionValue :type Boolean) (ElapsedSeconds :type "Float (double-precision)") (TriggeredSeconds :type "Float (double-precision)") (InputAction :type "InputAction Object Reference" :default "/Game/Input/Actions/Menu/IA_Inventory.IA_Inventory"))
  (bind _returnvalue (`GameplayStatics.GetPlayerController` 0))
  (bind _bp_maris (`self.BP Maris`))
  (bind _bp_maris_2 (`self.BP Maris`))
  (bind _bp_maris_3 (`self.BP Maris`))
  ;[0.07656 0.15 0 0.5] Inventory
  (:`Started`
    (`self.WBP Inventory`
      (:`then`
        (if (`Widget.IsVisible` (`self.WBP Inventory`))
          (`Widget.RemoveFromParent` (`self.WBP Inventory`))
          (`WidgetBlueprintLibrary.SetInputMode_GameOnly` _returnvalue)
          (set `PlayerController.bShowMouseCursor` false _returnvalue)
          (`CharacterMovementComponent.SetMovementMode` (`Character.CharacterMovement` _bp_maris_2) "MOVE_Walking" 0)
          (set `/Game/Blueprints/Maris/BP_Maris.CanCrouch?` true _bp_maris_2)
          (`SceneComponent.SetVisibility` (`/Game/Blueprints/Maris/BP_Maris.CharacterViewLight` _bp_maris_2) false false)
          (`self.SetActive` (`/Game/Blueprints/Maris/BP_Maris.EquipmentUICapture` _bp_maris_2) false false)
          (`KismetSystemLibrary.Delay` 0.15)
          (else
            (`self.SetActive` (`/Game/Blueprints/Maris/BP_Maris.EquipmentUICapture` _bp_maris_3) true false :!label _label)
            (`SceneComponent.SetVisibility` (`/Game/Blueprints/Maris/BP_Maris.CharacterViewLight` _bp_maris_3) true false)
            (`UserWidget.AddToViewport` (stale _output_get) 0)
            (`WidgetBlueprintLibrary.SetInputMode_GameAndUIEx` (`GameplayStatics.GetPlayerController` 0) (`self.WBP Inventory`))
            (set `PlayerController.bShowMouseCursor` true (`GameplayStatics.GetPlayerController` 0))
            (`/Game/UI/WBP_Inventory.UpdateInventory` (`self.WBP Inventory`) (`self.S_Slots`))
            (`CharacterMovementComponent.SetMovementMode` (`Character.CharacterMovement` _bp_maris) "MOVE_None" 0)
            (set `/Game/Blueprints/Maris/BP_Maris.CanCrouch?` false _bp_maris)
            (add `/Game/UI/WBP_Inventory.OnInventoryEquipped` (`self.WBP Inventory`) (delegate `UpdateEquipment`)))))
      (:`else`
        (bind _returnvalue_2 (`|CreateWidget` "/Game/UI/WBP_Inventory.WBP_Inventory_C" (`GameplayStatics.GetPlayerController` 0) (`self.S_Slots`)))
        (bind _output_get (set `self.WBP Inventory` _returnvalue_2))
        (goto _label)))))

(event `UpdateEquipment`
  (params (ItemData :type "/Game/Blueprints/InventorySystem/S_Items Structure"))
  ;[0.07656 0.15 0 0.5] Inventory
  (`self.UpdateEquipments` ItemData))

(fn `AddToInventory`
  (params (NewItem :type "/Game/Blueprints/InventorySystem/S_Slots Structure (by ref)"))
  (`KismetArrayLibrary.Array_Add` (`self.S_Slots`) NewItem))

(fn `EquipGun`
  (params (`Item Data` :type "/Game/Blueprints/InventorySystem/S_Items Structure"))
  (locals (WillEquipGun :type "/Game/Blueprints/InventorySystem/S_Items Structure"))
  (bind _equippedgun_name (break `/Game/Blueprints/InventorySystem/S_Items` (`self.EquippedGun`)))
  (if (`KismetStringLibrary.NotEqual_StrStr` (`.Name_2_5629E1A249ECBECC0478C3AEFAC0A9DE` (break `/Game/Blueprints/InventorySystem/S_Items` `Item Data`)) _equippedgun_name)
    (bind _output_get (set `self.EquippedGun` `Item Data`))
    (bind (_name _required_charisma _damageheal _icon _staticmesh _type _description _skeletalmeshsuit _amountrom) (break `/Game/Blueprints/InventorySystem/S_Items` _output_get))
    (`Image.SetBrushFromTexture` (`/Game/UI/WBP_Inventory.IMG_GunIcon` (`self.WBP Inventory`)) _icon true)
    (`StaticMeshComponent.SetStaticMesh` (`/Game/Blueprints/Maris/BP_Maris.PistolHand` (`self.BP Maris`)) _staticmesh)
    (set `self.IsGunEquipped` true)
    (set `self.GunFlints` _amountrom)))

(fn `EquipRom`
  (params (ItemData :type "/Game/Blueprints/InventorySystem/S_Items Structure"))
  (bind _equippedrom_name (break `/Game/Blueprints/InventorySystem/S_Items` (`self.EquippedRom`)))
  (if (`KismetStringLibrary.NotEqual_StrStr` (`.Name_2_5629E1A249ECBECC0478C3AEFAC0A9DE` (break `/Game/Blueprints/InventorySystem/S_Items` ItemData)) _equippedrom_name)
    (bind _output_get (set `self.EquippedRom` ItemData))
    (bind (_name _required_charisma _damageheal _icon _staticmesh _type _description _skeletalmeshsuit _amountrom) (break `/Game/Blueprints/InventorySystem/S_Items` _output_get))
    (`Image.SetBrushFromTexture` (`/Game/UI/WBP_Inventory.IMG_RomIcon` (`self.WBP Inventory`)) _icon true)
    (set `self.IsRomEquipped` true)
    (set `self.RomCapacity` _amountrom)))

(fn `EquipSling`
  (params (ItemData :type "/Game/Blueprints/InventorySystem/S_Items Structure"))
  (bind _equippedsling_name (break `/Game/Blueprints/InventorySystem/S_Items` (`self.EquippedSling`)))
  (if (`KismetStringLibrary.NotEqual_StrStr` _equippedsling_name (`.Name_2_5629E1A249ECBECC0478C3AEFAC0A9DE` (break `/Game/Blueprints/InventorySystem/S_Items` ItemData)))
    (bind _output_get (set `self.EquippedSling` ItemData))
    (bind (_name _required_charisma _damageheal _icon _staticmesh _type _description _skeletalmeshsuit _amountrom) (break `/Game/Blueprints/InventorySystem/S_Items` _output_get))
    (`Image.SetBrushFromTexture` (`/Game/UI/WBP_Inventory.IMG_SlingIcon` (`self.WBP Inventory`)) _icon true)
    (set `self.IsSlingEquipped` true)
    (set `self.SlingCapacity` _amountrom)))

(fn `EquipSuit`
  (params (ItemData :type "/Game/Blueprints/InventorySystem/S_Items Structure"))
  (bind _output_get (set `self.EquippedSuit` ItemData))
  (bind (_name _required_charisma _damageheal _icon _staticmesh _type _description _skeletalmeshsuit) (break `/Game/Blueprints/InventorySystem/S_Items` _output_get))
  (`Image.SetBrushFromTexture` (`/Game/UI/WBP_Inventory.IMG_Suit` (`self.WBP Inventory`)) _icon true)
  (`SkeletalMeshComponent.SetSkeletalMeshAsset` (`Character.Mesh` (`self.BP Maris`)) _skeletalmeshsuit))

(fn `EquipSword`
  (params (`Item Data` :type "/Game/Blueprints/InventorySystem/S_Items Structure"))
  (bind _img_swordicon (`/Game/UI/WBP_Inventory.IMG_SwordIcon` (`self.WBP Inventory`)))
  (bind _output_get (set `self.EquippedSword` `Item Data`))
  (bind (_name _required_charisma _damageheal _icon _staticmesh) (break `/Game/Blueprints/InventorySystem/S_Items` _output_get))
  (`Image.SetBrushFromTexture` _img_swordicon _icon false)
  (`Image.SetDesiredSizeOverride` _img_swordicon (50.0 25.0))
  (`StaticMeshComponent.SetStaticMesh` (`/Game/Blueprints/Maris/BP_Maris.SwordMeshSocket` (`self.BP Maris`)) _staticmesh)
  (set `self.IsSwordEquipped` true))

(fn `StoreKeyVariables`
  (bind _asbp_maris (cast `/Game/Blueprints/Maris/BP_Maris` (`self.GetOwner`)))
  (bind _output_get (set `self.BP Maris` _asbp_maris))
  (set `self.Follow Camera` (`/Game/Blueprints/Maris/BP_Maris.FollowCamera` _output_get)))

(fn `UpdateEquipments`
  (params (ItemData :type "/Game/Blueprints/InventorySystem/S_Items Structure"))
  (switch `/Game/Blueprints/InventorySystem/E_ItemTypes` (`.Type_18_6874192A4834BD09ECE5B5AD8FBF05BD` (break `/Game/Blueprints/InventorySystem/S_Items` ItemData))
    (:`NewEnumerator0`
      (`self.EquipSword` ItemData))
    (:`NewEnumerator1`
      (`self.EquipGun` ItemData))
    (:`NewEnumerator2`
      (`self.EquipSuit` ItemData))
    (:`NewEnumerator3`
      (`self.EquipRom` ItemData))
    (:`NewEnumerator4`
      (`self.EquipSling` ItemData))))