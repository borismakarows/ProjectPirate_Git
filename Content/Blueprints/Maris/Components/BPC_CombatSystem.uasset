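; Combat component for the Maris player character, handling sword combos, guard and parry, gun shots and evade.
; Montage notifies open combo, parry, block, roll and invincibility windows, with do-once gates and continue flags chaining combo and back-step-into-roll inputs.
; Melee sphere traces and gun line traces send damage through stat interface messages and report damage events to AI.
; Parry launches the target and briefly slows time.
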(event `self.ReceiveBeginPlay`
  (`self.StoreKeyVariables`))

(event `EnhancedInput|/Game/Input/Actions/Combat/IA_Guard`
  (params (ActionValue :type Boolean) (ElapsedSeconds :type "Float (double-precision)") (TriggeredSeconds :type "Float (double-precision)") (InputAction :type "InputAction Object Reference" :default "/Game/Input/Actions/Combat/IA_Guard.IA_Guard"))
  ; Guard Input
  (:`Started`
    (`self.StartBlock`))
  (:`Canceled`
    (`self.EndBlock` :!label _label))
  (:`Completed`
    (goto _label)))

(event `ShootToLockedEnemy`
  (params (AttackTarget :type "Actor Object Reference"))
  (bind _returnvalue (`Actor.K2_GetActorLocation` AttackTarget))
  (bind _bp_maris (`self.BP_Maris`))
  (bind _bp_maris_2 (`self.BP_Maris`))
  (bind _returnvalue_2 (`Actor.K2_GetActorLocation` (`self.BP_Maris`)))
  ;[0.009603 0.01042 0.01017] ShootToLockedEnemy
  (set `/Game/Blueprints/Maris/BP_Maris.CanMove?` false _bp_maris_2)
  (`Actor.K2_SetActorRotation` _bp_maris_2 (`KismetMathLibrary.FindLookAtRotation` (`Actor.K2_GetActorLocation` _bp_maris_2) (`Actor.K2_GetActorLocation` AttackTarget)) false)
  (bind _notifyname (`|PlayMontage` (`self.CharacterSKM`) "/Game/Assets/Maris/Animation/Gun/ShootingGun_Montage.ShootingGun_Montage" 1.2)
    (:`OnCompleted`
      (set `/Game/Blueprints/Maris/BP_Maris.CanMove?` true (`self.BP_Maris`) :!label _label_2))
    (:`OnInterrupted`
      (goto _label_2))
    (:`OnNotifyBegin`
      (switch `name` _notifyname
        (:`Shoot`
          (if (<= (`KismetMathLibrary.Vector_Distance2D` _returnvalue_2 _returnvalue) (`self.GunRange`))
            (bind (_outhit _returnvalue_3) (`KismetSystemLibrary.LineTraceSingle` :`Start` _returnvalue_2 :`End` _returnvalue :`TraceChannel` "TraceTypeQuery1" :`DrawDebugType` "ForDuration"))
            (if _returnvalue_3
              (bind (_bblockinghit _binitialoverlap _time _distance _location _impactpoint _normal _impactnormal _physmat _hitactor) (`GameplayStatics.BreakHitResult` _outhit))
              (if (`KismetSystemLibrary.DoesImplementInterface` _hitactor "/Game/Blueprints/DamageSystem/BPI_StatManagement.BPI_StatManagement_C")
                (message `/Game/Blueprints/DamageSystem/BPI_StatManagement.TakeDamage` _hitactor (make `/Game/Blueprints/DamageSystem/S_DamageInfo` 25.0 "NewEnumerator2" "NewEnumerator1" false false false false _bp_maris))
                (`AISense_Damage.ReportDamageEvent` _hitactor _bp_maris 25.0 _impactpoint)))))))))

(event `StartBlock`
  (bind _bp_maris (`self.BP_Maris`))
  ;[0 0 0] Guard
  ;; Start Block
  (if (and (`/Game/Blueprints/Maris/Components/BPC_InventorySystem.IsSwordEquipped` (`/Game/Blueprints/Maris/BP_Maris.BPC_InventorySystem` _bp_maris)) (not (`/Game/Blueprints/Maris/Components/BPC_Stats.IsStaminaDepleted?` (`/Game/Blueprints/Maris/BP_Maris.BPC_Stats` _bp_maris))))
    (`/Engine/EditorBlueprintResources/StandardMacros.DoOnce` false :!label _label_3
      (:`Completed`
        (set `/Game/Blueprints/Maris/BP_Maris.CanMove?` false (`self.BP_Maris`))
        (bind _notifyname (`|PlayMontage` (`self.CharacterSKM`) "/Game/Assets/Maris/Animation/Guard/ParryandBlock_Montage.ParryandBlock_Montage")
          (:`OnCompleted`
            (`self.EndBlock` :!label _label_4))
          (:`OnInterrupted`
            (goto _label_4))
          (:`OnNotifyBegin`
            (switch `name` _notifyname
              (:`Block`
                (set `/Game/Blueprints/Maris/Components/BPC_Stats.IsBlocking` true (`/Game/Blueprints/Maris/BP_Maris.BPC_Stats` (`self.BP_Maris`))))
              (:`ParryWindow`
                (set `self.WithinParryWindow?` true))))
          (:`OnNotifyEnd`
            (switch `name` _notifyname
              (:`ParryWindow`
                (set `self.WithinParryWindow?` false)))))))))

(event `EndBlock`
  ;[0 0 0] Guard
  ;; End Block
  (set `/Game/Blueprints/Maris/Components/BPC_Stats.IsBlocking` false (`/Game/Blueprints/Maris/BP_Maris.BPC_Stats` (`self.BP_Maris`)))
  (`self.ResetBlock`)
  (`Character.StopAnimMontage` (`self.BP_Maris`) "/Game/Assets/Maris/Animation/Guard/ParryandBlock_Montage.ParryandBlock_Montage")
  (set `self.WithinParryWindow?` false)
  (set `/Game/Blueprints/Maris/BP_Maris.CanMove?` true (`self.BP_Maris`)))

(event `ResetBlock`
  ;[0 0 0] Guard
  ;; Start Block
  (goto _label_3 :!via `Reset`))

(event `ShootToFront`
  (bind _bp_maris (`self.BP_Maris`))
  (bind _bp_maris_2 (`self.BP_Maris`))
  (bind _bp_maris_3 (`self.BP_Maris`))
  (bind _returnvalue (`Actor.K2_GetActorLocation` _bp_maris))
  ;[0.009603 0.01042 0.01017] ShotToFront
  (set `/Game/Blueprints/Maris/BP_Maris.CanMove?` false _bp_maris_2)
  (`/Game/Blueprints/Maris/Components/BPC_StateManager.SetStateFreeCombat` (`/Game/Blueprints/Maris/BP_Maris.BPC_StateManager` _bp_maris_2))
  (bind _notifyname (`|PlayMontage` (`self.CharacterSKM`) "/Game/Assets/Maris/Animation/Gun/ShootingGun_Montage.ShootingGun_Montage" 1.2)
    (:`OnCompleted`
      (set `/Game/Blueprints/Maris/BP_Maris.CanMove?` true (`self.BP_Maris`) :!label _label_5))
    (:`OnInterrupted`
      (goto _label_5))
    (:`OnNotifyBegin`
      (switch `name` _notifyname
        (:`Shoot`
          (bind (_outhit _returnvalue_2) (`KismetSystemLibrary.LineTraceSingle` _returnvalue (+ _returnvalue (* (`Actor.GetActorForwardVector` _bp_maris) (`self.GunRange`))) "TraceTypeQuery1" false (`|MakeArray` (`self.BP_Maris`) :!type "Actor Object Reference") "ForDuration"))
          (if _returnvalue_2
            (bind (_bblockinghit _binitialoverlap _time _distance _location _impactpoint _normal _impactnormal _physmat _hitactor) (`GameplayStatics.BreakHitResult` _outhit))
            (if (`KismetSystemLibrary.DoesImplementInterface` _hitactor "/Game/Blueprints/DamageSystem/BPI_StatManagement.BPI_StatManagement_C")
              (message `/Game/Blueprints/DamageSystem/BPI_StatManagement.TakeDamage` _hitactor (make `/Game/Blueprints/DamageSystem/S_DamageInfo` 25.0 "NewEnumerator2" "NewEnumerator1" false false false false _bp_maris_3))
              (`AISense_Damage.ReportDamageEvent` _hitactor _bp_maris_3 25.0 _impactpoint))))))))

(event `Parry`
  (params (AttackTarget :type "Actor Object Reference"))
  ;[0 0 0] Guard
  ;;[1 0.1067 0] Parry
  (message `/Game/Blueprints/DamageSystem/BPI_StatManagement.LaunchActor` AttackTarget (* (`self.LaunchScale`) (`Actor.GetActorForwardVector` (`self.BP_Maris`))) true false)
  (message `/Game/Blueprints/DamageSystem/BPI_StatManagement.TakeDamage` AttackTarget (make `/Game/Blueprints/DamageSystem/S_DamageInfo` 1.0 "NewEnumerator1" "NewEnumerator2" true false false true (`self.BP_Maris`)))
  (`KismetSystemLibrary.Delay` 0.2)
  (`GameplayStatics.SetGlobalTimeDilation` 0.2)
  (`KismetSystemLibrary.Delay` 0.1)
  (`GameplayStatics.SetGlobalTimeDilation` 1.0))

(event `EnhancedInput|/Game/Input/Actions/Combat/IA_Attack`
  (params (ActionValue :type Boolean) (ElapsedSeconds :type "Float (double-precision)") (TriggeredSeconds :type "Float (double-precision)") (InputAction :type "InputAction Object Reference" :default "/Game/Input/Actions/Combat/IA_Attack.IA_Attack"))
  (bind _bp_maris (`self.BP_Maris`))
  (bind _bp_maris_2 (`self.BP_Maris`))
  (bind _bpc_stats (`/Game/Blueprints/Maris/BP_Maris.BPC_Stats` _bp_maris))
  ;[0.15 0 0.003356 0.5] Combo Attack
  ;; Combat Input
  (:`Started`
    (`/Game/Blueprints/Maris/BP_Maris.EnemyToLock` _bp_maris_2
      (:`then`
        _)
      (:`else`
        (`/Game/Blueprints/Maris/Components/BPC_StateManager.SetStateFreeCombat` (`/Game/Blueprints/Maris/BP_Maris.BPC_StateManager` _bp_maris_2))))
    (if (and (`self.CanAttack`) (> (`/Game/Blueprints/Maris/Components/BPC_Stats.CurrentStamina` _bpc_stats) (`self.ComboStaminaDepValue`)) (not (`/Game/Blueprints/Maris/Components/BPC_Stats.IsStaminaDepleted?` _bpc_stats)) (`/Game/Blueprints/Maris/Components/BPC_InventorySystem.IsSwordEquipped` (`/Game/Blueprints/Maris/BP_Maris.BPC_InventorySystem` _bp_maris)))
      (`self.AttackCombo`))))

(event `EnhancedInput|/Game/Input/Actions/Combat/IA_Evade`
  (params (ActionValue :type Boolean) (ElapsedSeconds :type "Float (double-precision)") (TriggeredSeconds :type "Float (double-precision)") (InputAction :type "InputAction Object Reference" :default "/Game/Input/Actions/Combat/IA_Evade.IA_Evade"))
  ;[0 0.6598 0.7083 0.5] Evade
  (:`Started`
    (if (not (`/Game/Blueprints/Maris/Components/BPC_Stats.IsStaminaDepleted?` (`/Game/Blueprints/Maris/BP_Maris.BPC_Stats` (`self.BP_Maris`))))
      (`self.Evade`))))

(event `AttackCombo`
  ;[0.15 0 0.003356 0.5] Combo Attack
  ;; Attack Combo
  (`/Engine/EditorBlueprintResources/StandardMacros.DoOnce` false :!label _label_6
    (:`Completed`
      (if (not (`self.WithinComboWindow?`))
        (bind _notifyname (`|PlayMontage` (`self.CharacterSKM`) "/Game/Assets/Maris/Animation/Attack/Maris_SwordCombo.Maris_SwordCombo")
          (:`then`
            (set `/Game/Blueprints/Maris/BP_Maris.IsConsumingStamina?` true (`self.BP_Maris`)))
          (:`OnCompleted`
            (set `/Game/Blueprints/Maris/BP_Maris.IsConsumingStamina?` false (`self.BP_Maris`) :!label _label_7)
            (set `self.ContinueToCombo` false)
            (`self.ResetCombo`))
          (:`OnInterrupted`
            (goto _label_7))
          (:`OnNotifyBegin`
            (switch `name` _notifyname
              (:`Hit`
                (`self.MeleeDamage` 130.0 (make `/Game/Blueprints/DamageSystem/S_DamageInfo` 20.0 "NewEnumerator1" "NewEnumerator1" false true false false (`self.BP_Maris`))))
              (:`SmallHit`
                (`self.MeleeDamage` 75.0 (make `/Game/Blueprints/DamageSystem/S_DamageInfo` 10.0 "NewEnumerator1" "NewEnumerator1" false true false false (`self.BP_Maris`))))
              (:`ContinueCombo`
                (set `self.WithinComboWindow?` true)
                (set `self.ContinueToCombo` false)
                (`self.ResetCombo`))))
          (:`OnNotifyEnd`
            (switch `name` _notifyname
              (:`ContinueCombo`
                (set `self.WithinComboWindow?` false)
                (if (not (`self.ContinueToCombo`))
                  (`Character.StopAnimMontage` (`self.BP_Maris`) "/Game/Assets/Maris/Animation/Attack/Maris_SwordCombo.Maris_SwordCombo"))))))
        (else
          (set `self.ContinueToCombo` true))))))

(event `ResetCombo`
  ;[0.15 0 0.003356 0.5] Combo Attack
  ;; Attack Combo
  (goto _label_6 :!via `Reset`))

(event `Evade`
  (bind _bpc_stats (`/Game/Blueprints/Maris/BP_Maris.BPC_Stats` (`self.BP_Maris`)))
  (bind _bpc_stats_2 (`/Game/Blueprints/Maris/BP_Maris.BPC_Stats` (`self.BP_Maris`)))
  ;[0 0.6598 0.7083 0.5] Evade
  (if (not (`self.WithinRollWindow?`))
    (`/Engine/EditorBlueprintResources/StandardMacros.DoOnce` false :!label _label_8
      (:`Completed`
        (if (not (`self.IsAttacking`))
          (bind _notifyname (`|PlayMontage` (`self.CharacterSKM`) "/Game/Assets/Maris/Animation/Evade/BackStep_Roll_Montage.BackStep_Roll_Montage")
            (:`OnCompleted`
              (`self.ResetEvade` :!label _label_9)
              (set `self.ContinueToRoll` false)
              (set `/Game/Blueprints/Maris/BP_Maris.IsConsumingStamina?` false (`self.BP_Maris`)))
            (:`OnInterrupted`
              (goto _label_9))
            (:`OnNotifyBegin`
              (switch `name` _notifyname
                (:`BackStep`
                  (`/Game/Blueprints/Maris/BP_Maris.StaminaDeplete` (`self.BP_Maris`) (`self.EvadeStaminaDeplete`))
                  (set `/Game/Blueprints/Maris/BP_Maris.IsConsumingStamina?` true (`self.BP_Maris`)))
                (:`iFrame`
                  (set `/Game/Blueprints/Maris/Components/BPC_Stats.IsInvincible` true _bpc_stats_2)
                  (set `/Game/Blueprints/Maris/Components/BPC_Stats.IsInterruptible` false _bpc_stats_2))
                (:`RollWindow`
                  (set `self.WithinRollWindow?` true))
                (:`Roll`
                  (`/Game/Blueprints/Maris/BP_Maris.StaminaDeplete` (`self.BP_Maris`) (`self.EvadeStaminaDeplete`)))))
            (:`OnNotifyEnd`
              (switch `name` _notifyname
                (:`iFrame`
                  (set `/Game/Blueprints/Maris/Components/BPC_Stats.IsInvincible` false _bpc_stats)
                  (set `/Game/Blueprints/Maris/Components/BPC_Stats.IsInterruptible` true _bpc_stats))
                (:`RollWindow`
                  (set `self.WithinRollWindow?` false)
                  (if (not (`self.ContinueToRoll`))
                    (`Character.StopAnimMontage` (`self.BP_Maris`) "/Game/Assets/Maris/Animation/Evade/BackStep_Roll_Montage.BackStep_Roll_Montage")))))))))
    (else
      (set `self.ContinueToRoll` true))))

(event `ResetEvade`
  ;[0 0.6598 0.7083 0.5] Evade
  (goto _label_8 :!via `Reset`))

(event `MeleeDamage`
  (params (AttackRange :type "Float (double-precision)") (DamageInfo :type "/Game/Blueprints/DamageSystem/S_DamageInfo Structure"))
  (bind (_amount _damagetype _damageresponse _shoulddamageinvincible _canbeblocked _canbeparried _shouldforceinterrupt _damagecauser) (break `/Game/Blueprints/DamageSystem/S_DamageInfo` DamageInfo))
  ;[1 0.4181 0 0.5] Melee Damage
  (bind (_hitresults _hit_) (`self.MultiSphereTrace` AttackRange))
  (if _hit_
    (bind _damagedactors (`self.DamageAllNonTeamMembers` _hitresults DamageInfo))
    (bind _output (`|GetArrayItem` _damagedactors))
    (`AISense_Damage.ReportDamageEvent` _output _damagecauser 25.0 (`Actor.K2_GetActorLocation` _damagecauser))
    (message `/Game/Blueprints/DamageSystem/BPI_StatManagement.LaunchActor` _output (* (`self.LaunchScale`) (`Actor.GetActorForwardVector` (`self.BP_Maris`))) true false)
    (`GameplayStatics.PlayWorldCameraShake` "/Game/Blueprints/Maris/BP_EnemyHitCameraShake.BP_EnemyHitCameraShake_C" (0.0 0.0 0.0) 0.0 2000.0)))

(fn `DamageAllNonTeamMembers`
  (params (Hits :type "Array of HitResult Structure") (DamageInfo :type "/Game/Blueprints/DamageSystem/S_DamageInfo Structure"))
  (returns (DamagedActors :type "Array of Actor Object Reference"))
  (locals (ActorDamageSoFar :type "Array of Actor Object Reference"))
  (bind _actordamagesofar (`local.ActorDamageSoFar`))
  (for _array_element Hits
    (bind (_bblockinghit _binitialoverlap _time _distance _location _impactpoint _normal _impactnormal _physmat _hitactor) (`GameplayStatics.BreakHitResult` _array_element))
    (bind _sameteam (`self.OnSameTeam` _hitactor))
    (if (and (not _sameteam) (not (`KismetArrayLibrary.Array_Contains` _actordamagesofar _hitactor)))
      (message `/Game/Blueprints/DamageSystem/BPI_StatManagement.TakeDamage` _hitactor DamageInfo)
      (`KismetArrayLibrary.Array_AddUnique` (`local.ActorDamageSoFar`) _hitactor)))
  (return _actordamagesofar))

(fn `DamageFirstNonTeamMembers`
  (params (Hits :type "Array of HitResult Structure") (`Damage Info` :type "/Game/Blueprints/DamageSystem/S_DamageInfo Structure"))
  (returns (DamagedActor :type "Actor Object Reference"))
  (for _array_element Hits
    (bind (_bblockinghit _binitialoverlap _time _distance _location _impactpoint _normal _impactnormal _physmat _hitactor) (`GameplayStatics.BreakHitResult` _array_element))
    (bind _sameteam (`self.OnSameTeam` _hitactor))
    (if (not _sameteam)
      (message `/Game/Blueprints/DamageSystem/BPI_StatManagement.TakeDamage` _hitactor `Damage Info`)
      (`|ExecutionSequence`
        (:`then_0`
          (break))
        (:`then_1`
          (return _hitactor))))))

(fn `MultiSphereTrace`
  (params (AttackRange :type "Float (double-precision)") (AttackTarget :type "Actor Object Reference"))
  (returns (HitResults :type "Array of HitResult Structure") (`Hit?` :type Boolean))
  (locals (EndLoc :type "Vector Structure" :default (0.0 0.0 0.0)))
  (bind _returnvalue (`self.GetOwner`))
  (`local.AttackTarget`
    (:`then`
      (set `local.EndLoc` (`Actor.K2_GetActorLocation` (`local.AttackTarget`)))
      (if (not (>= (`local.AttackRange`) (`KismetMathLibrary.Vector_Distance2D` (`Actor.K2_GetActorLocation` (`self.GetOwner`)) (`local.EndLoc`))))
        (set `local.EndLoc` (+ (`Actor.K2_GetActorLocation` _returnvalue) (* (`Actor.GetActorForwardVector` _returnvalue) (`local.AttackRange`))) :!label _label)))
    (:`else`
      (goto _label)))
  (bind (_outhits _returnvalue_2) (`KismetSystemLibrary.SphereTraceMulti` (`Actor.K2_GetActorLocation` (`self.GetOwner`)) (`local.EndLoc`) 8.0 "TraceTypeQuery1" false (`|MakeArray` (`self.GetOwner`) (`self.BP_Maris`) :!type "Actor Object Reference") "ForDuration"))
  (return _outhits _returnvalue_2))

(fn `OnSameTeam`
  (params (Actor :type "Actor Object Reference"))
  (returns (SameTeam :type Boolean))
  (bind _teamnumber (message `/Game/Blueprints/DamageSystem/BPI_StatManagement.GetTeamNumber` Actor))
  (bind _teamnumber_2 (message `/Game/Blueprints/DamageSystem/BPI_StatManagement.GetTeamNumber` (`self.GetOwner`)))
  (return (== _teamnumber_2 _teamnumber)))

(fn `StoreKeyVariables`
  (bind _asbp_maris (cast `/Game/Blueprints/Maris/BP_Maris` (`self.GetOwner`)))
  (bind _output_get (set `self.BP_Maris` _asbp_maris))
  (set `self.CharacterSKM` (`Character.Mesh` _output_get)))