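; Player component for Maris that switches between roaming, free combat and locked combat states.
; Each state setter updates the state enum, HUD visibility and max walk speed.
; Locked combat starts a fast looping timer, apparently driving TargetLockRotation, which aims control rotation at the locked enemy and makes movement follow it.
; CancelLock clears the target and timer, restores movement-oriented rotation and returns to free combat; SetStanceDefault is an empty stub.
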(event `self.ReceiveBeginPlay`
  (bind _asbp_maris (cast `/Game/Blueprints/Maris/BP_Maris` (`GameplayStatics.GetPlayerCharacter` 0)))
  (set `self.MarisRef` _asbp_maris))

(event `TargetLockRotation`
  (bind _marisref (`self.MarisRef`))
  (bind _charactermovement (`Character.CharacterMovement` (`self.MarisRef`)))
  ; Rotation of Target Lock
  (bind _enemytolock (`/Game/Blueprints/Maris/BP_Maris.EnemyToLock` (`self.MarisRef`))
    (:`then`
      (`Controller.SetControlRotation` (`Pawn.GetController` _marisref) (`KismetMathLibrary.FindLookAtRotation` (`SceneComponent.K2_GetComponentLocation` (`Character.CapsuleComponent` _marisref)) (- (`Actor.K2_GetActorLocation` _enemytolock) (0.0 0.0 100.0))))
      (set `CharacterMovementComponent.bOrientRotationToMovement` false _charactermovement)
      (set `CharacterMovementComponent.bUseControllerDesiredRotation` true _charactermovement))
    (:`else`)))

(fn `CancelLock`
  (bind _marisref (`self.MarisRef`))
  (bind _charactermovement (`Character.CharacterMovement` _marisref))
  (set `/Game/Blueprints/Maris/BP_Maris.EnemyToLock` null _marisref)
  (set `CharacterMovementComponent.bOrientRotationToMovement` true _charactermovement)
  (set `CharacterMovementComponent.bUseControllerDesiredRotation` false _charactermovement)
  (`KismetSystemLibrary.K2_ClearAndInvalidateTimerHandle` (`self.EnemyLockTimerHandle`))
  (`self.SetStateFreeCombat`))

(fn `SetStanceDefault`)

(fn `SetStateFreeCombat`
  (bind _marisref (`self.MarisRef`))
  (set `self.PlayerStates` "NewEnumerator1")
  (`Widget.SetVisibility` (`/Game/Blueprints/Maris/BP_Maris.WBP_Hud` _marisref) "Visible")
  (set `CharacterMovementComponent.MaxWalkSpeed` (`self.CombatMovementSpeed`) (`Character.CharacterMovement` _marisref)))

(fn `SetStateLockedCombat`
  (bind _marisref (`self.MarisRef`))
  (set `self.PlayerStates` "NewEnumerator2")
  (`Widget.SetVisibility` (`/Game/Blueprints/Maris/BP_Maris.WBP_Hud` _marisref) "Visible")
  (set `CharacterMovementComponent.MaxWalkSpeed` (`self.LockedMovementSpeed`) (`Character.CharacterMovement` _marisref))
  (bind _returnvalue (`KismetSystemLibrary.K2_SetTimerDelegate` (`|CreateDelegate` :!event `TargetLockRotation`) 0.01 true))
  (set `self.EnemyLockTimerHandle` _returnvalue))

(fn `SetStateRoaming`
  (bind _marisref (`self.MarisRef`))
  (set `self.PlayerStates` "NewEnumerator0")
  (`Widget.SetVisibility` (`/Game/Blueprints/Maris/BP_Maris.WBP_Hud` _marisref) "Hidden")
  (set `CharacterMovementComponent.MaxWalkSpeed` (`self.UnarmedMovementSpeed`) (`Character.CharacterMovement` _marisref))
  (`KismetSystemLibrary.K2_ClearAndInvalidateTimerHandle` (`self.EnemyLockTimerHandle`)))