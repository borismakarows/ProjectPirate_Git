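; Player stance component for Maris that switches between roaming, free combat, locked combat and blocking.
; Each stance sets walk speed, with the HUD hidden when roaming and shown in combat.
; Locked combat runs a fast looping timer, apparently driving the control rotation toward the locked enemy, until the lock is cancelled.
; Free combat starts a periodic sphere trace for living enemies that can drop the stance back to roaming.
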(event `self.ReceiveBeginPlay`
  (bind _asbp_maris (cast `/Game/Blueprints/Maris/BP_Maris` (`GameplayStatics.GetPlayerCharacter` 0)))
  (set `self.MarisRef` _asbp_maris))

(event `TargetLockRotation`
  (bind _marisref (`self.MarisRef`))
  (bind _charactermovement (`Character.CharacterMovement` (`self.MarisRef`)))
  ; Rotation of Target Lock
  (bind _enemytolock (`/Game/Blueprints/Maris/BP_Maris.EnemyToLock` (`self.MarisRef`))
    (:`then`
      (`Controller.SetControlRotation` (`Pawn.GetController` _marisref) (`KismetMathLibrary.FindLookAtRotation` (`SceneComponent.K2_GetComponentLocation` (`Character.CapsuleComponent` _marisref)) (- (`Actor.K2_GetActorLocation` _enemytolock) (0.0 0.0 100.0))))
      (set `CharacterMovementComponent.bOrientRotationToMovement` false _charactermovement)
      (set `CharacterMovementComponent.bUseControllerDesiredRotation` true _charactermovement))
    (:`else`)))

(fn `AreThereAliveEnemiesAround`
  (locals (AliveEnemies :type "Array of Actor Object Reference"))
  (bind _returnvalue (`Actor.K2_GetActorLocation` (`self.MarisRef`)))
  (bind (_outhits _returnvalue_2) (`KismetSystemLibrary.SphereTraceMultiForObjects` _returnvalue _returnvalue 1500.0 (`|MakeArray` "ObjectTypeQuery7" :!type "EObjectTypeQuery Enum") false (`|MakeArray` (`self.MarisRef`) :!type "Actor Object Reference") "ForDuration"))
  (if _returnvalue_2
    (for _array_element _outhits
      (bind (_maxhealth _currenthealth _isdead_) (message `/Game/Blueprints/DamageSystem/BPI_StatManagement.GetHealthValues` (`.HitActor` (`GameplayStatics.BreakHitResult` _array_element))))
      (if (not _isdead_)
        (`KismetArrayLibrary.Array_Add` (`local.AliveEnemies`))))
    (if (== (`KismetArrayLibrary.Array_Length` (`local.AliveEnemies`)) 0)
      (`self.SetStanceRoaming`))))

(fn `CancelLock`
  (bind _marisref (`self.MarisRef`))
  (bind _charactermovement (`Character.CharacterMovement` _marisref))
  (message `/Game/Blueprints/Interfaces/BPI_TargetLock.SetUIOn_Off` (`/Game/Blueprints/Maris/BP_Maris.EnemyToLock` _marisref) false)
  (set `/Game/Blueprints/Maris/BP_Maris.EnemyToLock` null _marisref)
  (set `CharacterMovementComponent.bOrientRotationToMovement` true _charactermovement)
  (set `CharacterMovementComponent.bUseControllerDesiredRotation` false _charactermovement)
  (`KismetSystemLibrary.K2_ClearAndInvalidateTimerHandle` (`self.EnemyLockTimerHandle`))
  (`self.SetStanceFreeCombat`))

(fn `SetMovementSpeed`
  (params (MovementSpeed :type "/Game/Blueprints/Maris/Enums/E_PlayerMovementSpeed Enum" :default "NewEnumerator0"))
  (returns (Speed :type "Float (double-precision)"))
  (bind _output_get (set `CharacterMovementComponent.MaxWalkSpeed` (select `/Game/Blueprints/Maris/Enums/E_PlayerMovementSpeed` MovementSpeed :`NewEnumerator0` (`self.RoamingMovementSpeed`) :`NewEnumerator1` (`self.CombatMovementSpeed`) :`NewEnumerator2` (`self.LockedMovementSpeed`) :`NewEnumerator3` (`self.RomDrinkingMovementSpeed`) :`NewEnumerator4` (`self.BlockMovementSpeed`)) (`Character.CharacterMovement` (`self.MarisRef`))))
  (return _output_get))

(fn `SetStanceBlock`
  (`self.SetStanceFreeCombat`)
  (set `self.PlayerStance` "NewEnumerator3")
  (`self.SetMovementSpeed` "NewEnumerator4"))

(fn `SetStanceFreeCombat`
  (set `self.PlayerStance` "NewEnumerator1")
  (`Widget.SetVisibility` (`/Game/Blueprints/Maris/BP_Maris.WBP_Hud` (`self.MarisRef`)) "Visible")
  (`self.SetMovementSpeed` "NewEnumerator1")
  (bind _returnvalue (`KismetSystemLibrary.K2_SetTimer` null "AreThereAliveEnemiesAround" 30.0 true))
  (set `self.AreThereAliveEnemiesAroundTimerHandle` _returnvalue))

(fn `SetStanceLockedCombat`
  (`/Game/Blueprints/Maris/BP_Maris.EnemyToLock` (`self.MarisRef`)
    (:`then`
      (set `self.PlayerStance` "NewEnumerator2")
      (`Widget.SetVisibility` (`/Game/Blueprints/Maris/BP_Maris.WBP_Hud` (`self.MarisRef`)) "Visible")
      (`self.SetMovementSpeed` "NewEnumerator2")
      (bind _returnvalue (`KismetSystemLibrary.K2_SetTimerDelegate` (`|CreateDelegate` :!event `TargetLockRotation`) 0.001 true))
      (set `self.EnemyLockTimerHandle` _returnvalue))
    (:`else`
      (`self.SetStanceFreeCombat`))))

(fn `SetStanceRoaming`
  (set `self.PlayerStance` "NewEnumerator0")
  (`Widget.SetVisibility` (`/Game/Blueprints/Maris/BP_Maris.WBP_Hud` (`self.MarisRef`)) "Hidden")
  (`self.SetMovementSpeed` "NewEnumerator0")
  (`KismetSystemLibrary.K2_ClearAndInvalidateTimerHandle` (`self.EnemyLockTimerHandle`)))