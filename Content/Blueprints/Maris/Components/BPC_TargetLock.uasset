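; Target-lock component for the Maris player character that finds lockable enemies and switches the lock between them.
; TargetsTrace sphere-traces along the follow camera to cache living targets; FindClosestTarget picks the nearest by visibility line traces.
; Mouse input past a dead zone splits cached targets left/right by cross-product sign, then sets EnemyToLock to the nearest other one, with per-side cooldowns.
; Line traces hitting dead actors cancel the lock.
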(event `self.ReceiveBeginPlay`
  (bind _asbp_maris (cast `/Game/Blueprints/Maris/BP_Maris` (`GameplayStatics.GetPlayerCharacter` 0)))
  (set `self.BP_Maris` _asbp_maris))

(event `ChangeTargetWithMouseInput`
  (params (MouseInput :type "Float (double-precision)"))
  ; > Left input < Right input
  (`self.CompareWithErrorMargin` 0.0 MouseInput 0.5
    (:`>`
      (`/Engine/EditorBlueprintResources/StandardMacros.DoOnce` false :!label _label
        (:`Completed`
          (bind _targetsofdirection (`self.FindTargetsDirections` "Left"))
          (bind _enemytolock (`self.FindClosestTargetExceptLocked` _targetsofdirection))
          (if (`KismetSystemLibrary.IsValid` _enemytolock)
            (set `/Game/Blueprints/Maris/BP_Maris.EnemyToLock` _enemytolock (`self.BP_Maris`)))
          (`KismetSystemLibrary.Delay` 1.0)
          (goto _label :!via `Reset`))))
    (:`<`
      (`/Engine/EditorBlueprintResources/StandardMacros.DoOnce` false :!label _label_2
        (:`Completed`
          (bind _targetsofdirection_2 (`self.FindTargetsDirections` "Right"))
          (bind _enemytolock_2 (`self.FindClosestTargetExceptLocked` _targetsofdirection_2))
          (if (`KismetSystemLibrary.IsValid` _enemytolock_2)
            (set `/Game/Blueprints/Maris/BP_Maris.EnemyToLock` _enemytolock_2 (`self.BP_Maris`)))
          (`KismetSystemLibrary.Delay` 1.0)
          (goto _label_2 :!via `Reset`))))))

(fn `FindClosestTarget`
  (params (Targets :type "Array of Actor Object Reference"))
  (returns (EnemyToLock :type "Actor Object Reference"))
  (locals (LocalDistance :type "Float (double-precision)" :default 10000.0) (LocalActor :type "Actor Object Reference"))
  (set `local.LocalDistance` 10000.0)
  (for _array_element Targets
    (bind (_outhit _returnvalue) (`KismetSystemLibrary.LineTraceSingle` (`SceneComponent.K2_GetComponentLocation` (`/Game/Blueprints/Maris/BP_Maris.FollowCamera` (`self.BP_Maris`))) (`Actor.K2_GetActorLocation` _array_element) "TraceTypeQuery1" false (`|MakeArray` (`self.BP_Maris`) :!type "Actor Object Reference") "ForDuration"))
    (if _returnvalue
      (bind (_bblockinghit _binitialoverlap _time _distance _location _impactpoint _normal _impactnormal _physmat _hitactor) (`GameplayStatics.BreakHitResult` _outhit))
      (bind (_maxhealth _currenthealth _isdead_) (message `/Game/Blueprints/DamageSystem/BPI_StatManagement.GetHealthValues` _hitactor))
      (if (not _isdead_)
        (if (< _distance (`local.LocalDistance`))
          (set `local.LocalDistance` _distance)
          (set `local.LocalActor` _hitactor))
        (else
          (`/Game/Blueprints/Maris/BP_Maris.CancelTargetLock` (`self.BP_Maris`))))))
  (return (`local.LocalActor`)))

(fn `FindClosestTargetExceptLocked`
  (params (Targets :type "Array of Actor Object Reference"))
  (returns (EnemyToLock :type "Actor Object Reference"))
  (locals (LockedDistance :type "Float (double-precision)") (LocalActor :type "Actor Object Reference"))
  (set `local.LockedDistance` 10000.0)
  (for _array_element Targets
    (bind (_outhit _returnvalue) (`KismetSystemLibrary.LineTraceSingle` (`SceneComponent.K2_GetComponentLocation` (`/Game/Blueprints/Maris/BP_Maris.FollowCamera` (`self.BP_Maris`))) (`Actor.K2_GetActorLocation` _array_element) "TraceTypeQuery1" false (`|MakeArray` (`self.BP_Maris`) :!type "Actor Object Reference") "ForDuration"))
    (if _returnvalue
      (bind (_bblockinghit _binitialoverlap _time _distance _location _impactpoint _normal _impactnormal _physmat _hitactor) (`GameplayStatics.BreakHitResult` _outhit))
      (if (!= (`/Game/Blueprints/Maris/BP_Maris.EnemyToLock` (`self.BP_Maris`)) _hitactor)
        (bind (_maxhealth _currenthealth _isdead_) (message `/Game/Blueprints/DamageSystem/BPI_StatManagement.GetHealthValues` _hitactor))
        (if (not _isdead_)
          (if (< _distance (`local.LockedDistance`))
            (set `local.LockedDistance` _distance)
            (set `local.LocalActor` _hitactor))
          (else
            (`/Game/Blueprints/Maris/BP_Maris.CancelTargetLock` (`self.BP_Maris`)))))))
  (return (`local.LocalActor`)))

(fn `FindTargetsDirections`
  (params (Direction :type "EDirection Enum" :default "Left"))
  (returns (TargetsOfDirection :type "Array of Actor Object Reference"))
  (locals (RightActors :type "Array of Actor Object Reference") (LeftActors :type "Array of Actor Object Reference"))
  (for _array_element (`self.Targets`)
    (bind (_returnvalue_x _returnvalue_y _returnvalue_z) (`KismetMathLibrary.BreakVector` (`KismetMathLibrary.Cross_VectorVector` (`SceneComponent.GetForwardVector` (`/Game/Blueprints/Maris/BP_Maris.FollowCamera` (`self.BP_Maris`))) (`KismetMathLibrary.Normal` (- (`Actor.K2_GetActorLocation` _array_element) (`Actor.K2_GetActorLocation` (`self.BP_Maris`)))))))
    (`/Engine/EditorBlueprintResources/StandardMacros.CompareFloat` _returnvalue_z
      (:`>`
        (`KismetArrayLibrary.Array_Add` (`local.RightActors`) _array_element))
      (:`<`
        (`KismetArrayLibrary.Array_Add` (`local.LeftActors`) _array_element))))
  (return (select `EDirection` Direction :`Left` (`local.LeftActors`) :`Right` (`local.RightActors`))))

(fn `TargetsTrace`
  (params (TargetDistance :type "Float (double-precision)"))
  (returns (Targets :type "Array of Actor Object Reference"))
  (locals (LocalTargets :type "Array of Actor Object Reference"))
  (bind _bp_maris (`self.BP_Maris`))
  (bind _mesh (`Character.Mesh` _bp_maris))
  (bind (_outhits _returnvalue) (`KismetSystemLibrary.SphereTraceMultiForObjects` (+ (* (`SceneComponent.GetForwardVector` (`/Game/Blueprints/Maris/BP_Maris.FollowCamera` _bp_maris)) 500.0) (`SceneComponent.K2_GetComponentLocation` _mesh) (0.0 0.0 120.0)) (+ (`SceneComponent.K2_GetComponentLocation` _mesh) (* (`KismetMathLibrary.GetForwardVector` (`SceneComponent.K2_GetComponentRotation` (`/Game/Blueprints/Maris/BP_Maris.FollowCamera` _bp_maris))) (`local.TargetDistance`)) (0.0 0.0 120.0)) 500.0 (`|MakeArray` "ObjectTypeQuery7" :!type "EObjectTypeQuery Enum") false (`|MakeArray` (`self.BP_Maris`) :!type "Actor Object Reference")))
  (if _returnvalue
    (for _array_element _outhits
      (bind (_bblockinghit _binitialoverlap _time _distance _location _impactpoint _normal _impactnormal _physmat _hitactor) (`GameplayStatics.BreakHitResult` _array_element))
      (bind (_maxhealth _currenthealth _isdead_) (message `/Game/Blueprints/DamageSystem/BPI_StatManagement.GetHealthValues` _hitactor))
      (if (not _isdead_)
        (`KismetArrayLibrary.Array_Add` (`local.LocalTargets`) _hitactor)))
    (bind _output_get (set `self.Targets` (`local.LocalTargets`)))
    (return _output_get)))