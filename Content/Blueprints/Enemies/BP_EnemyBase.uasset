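; Base enemy character providing AI-callable attack, sword wield and sheathe, patrol route, combat range and movement speed functions.
; Montage callbacks signal action completion, while delays time spawning the morningstar onto the hand socket and destroying it.
; An overlap volume shows a backstab prompt to BP_Maris, and Backstab returns positioning for a delayed death animation.
; Damage feeds a stats component, triggering hit reaction with knockback or ragdoll death with timed cleanup.
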(event `Ragdoll`
  ; Ragdoll
  (`KismetSystemLibrary.Delay` 2.5)
  (`PrimitiveComponent.SetSimulatePhysics` (`self.Mesh`) true))

(event `self.BackStabCollision.OnComponentBeginOverlap`
  (params (OverlappedComponent :type "PrimitiveComponent Object Reference") (OtherActor :type "Actor Object Reference") (OtherComp :type "PrimitiveComponent Object Reference") (OtherBodyIndex :type Integer) (bFromSweep :type Boolean) (SweepResult :type "HitResult Structure (by ref)"))
  ; BackstabVisibility when it is possible
  (if (`GameplayStatics.ObjectIsA` OtherActor "/Game/Blueprints/Maris/BP_Maris.BP_Maris_C")
    (`SceneComponent.SetVisibility` (`self.BackstabWidget`) true false)
    (else
      (`SceneComponent.SetVisibility` (`self.BackstabWidget`) false false :!label _label))))

(event `DefaultAttack`
  ;[0.8229 0 0.006893 0.5] AI Default Attack
  (`|PlayMontage` (`self.Mesh`) "/Game/Animations/Maris/Attack/Attack2_Montage.Attack2_Montage"
    (:`OnCompleted`
      _)
    (:`OnInterrupted`
      _))
  (`self.OnAttackEnd`))

(event `self.BackStabCollision.OnComponentEndOverlap`
  (params (OverlappedComponent :type "PrimitiveComponent Object Reference") (OtherActor :type "Actor Object Reference") (OtherComp :type "PrimitiveComponent Object Reference") (OtherBodyIndex :type Integer))
  ; BackstabVisibility when it is possible
  (if (`GameplayStatics.ObjectIsA` OtherActor "/Game/Blueprints/Maris/BP_Maris.BP_Maris_C")
    (goto _label)))

(event `WieldSword`
  ;[0.2314 0.4688 0 0.5] AI Wielding Sword
  (`|PlayMontage` (`self.Mesh`) "/Game/Animations/Enemy/Armed/WieldingSword_Montage.WieldingSword_Montage" -1.0 1.25
    (:`then`
      (`KismetSystemLibrary.Delay` 0.2)
      (bind _returnvalue (`|SpawnActorFromClass` "/Game/InventorySystem/Swords/BP_Morningstar.BP_Morningstar_C" (`self.GetTransform`) "Undefined" "MultiplyWithRoot" null (make `/Game/InventorySystem/S_Slots` (make `DataTableRowHandle` "/Game/InventorySystem/DB_Items.DB_Items" "Morningstar")) null))
      (bind _output_get (set `self.EnemySword` _returnvalue))
      (`self.K2_AttachToComponent` _output_get (`self.Mesh`) "Weaponhand_r" "SnapToTarget" "SnapToTarget" "SnapToTarget" true))
    (:`OnCompleted`
      (`self.OnWieldSwordEnd` :!label _label_2)
      (set `self.IsWieldingSword` true))
    (:`OnInterrupted`
      (goto _label_2))))

(event `SetLifeSpanAfterDied`
  ;[0.15 0.02805 0.02655 0.5] Turn off Widget and set Life Span after died
  (`SceneComponent.SetVisibility` (`self.BackstabWidget`) false false)
  (`self.SetLifeSpan` 600.0))

(event `DieAnimation`
  ;[0.07812 0.07812 0.07812 0.5] Play dead animation with delay
  (`KismetSystemLibrary.Delay` (`self.BackstabDieAnimationDelay`))
  (`self.PlayAnimMontage` "/Game/Animations/Maris/BackStab/BackStab_vic_UE_Montage.BackStab_vic_UE_Montage")
  (`self.DeadSettings`))

(event `SheathSword`
  ; SheathSword
  (`|PlayMontage` (`self.Mesh`) "/Game/Animations/Enemy/Armed/SheathingSword_Montage.SheathingSword_Montage"
    (:`then`
      (`KismetSystemLibrary.Delay` 1.05)
      (`self.K2_DestroyActor` (`self.EnemySword`)))
    (:`OnCompleted`
      (`self.OnSheatSwordEnd` :!label _label_3)
      (set `self.IsWieldingSword` false))
    (:`OnInterrupted`
      (goto _label_3))))

(event `self.ReceiveAnyDamage`
  (params (Damage :type "Float (single-precision)") (DamageType :type "DamageType Object Reference") (InstigatedBy :type "Controller Object Reference") (DamageCauser :type "Actor Object Reference"))
  (bind _hitreactions (`self.HitReactions`))
  ;[1 0.1067 0] Get Hit
  (bind _isdead (`/Game/Blueprints/Dummy/BPC_EnemyStats.GetDamageHealth` (`self.BPC_EnemyStats`) Damage))
  (if _isdead
    (message `/Game/Blueprints/Interfaces/BPI_TargetLock.CancelTargetLock` DamageCauser)
    (`self.DeadSettings`)
    (else
      (`self.PlayAnimMontage` (`|GetArrayItem` _hitreactions (`KismetMathLibrary.RandomIntegerInRange` 0 (- (`KismetArrayLibrary.Array_Length` _hitreactions) 1))))
      (`self.LaunchCharacter` self (* (`KismetMathLibrary.GetForwardVector` (`self.K2_GetActorRotation` DamageCauser)) (`self.HitBackSlip`)) false false))))

(fn `AI_Attack`
  (returns (BP_EnemyBase :type "/Game/Blueprints/Enemies/BP_EnemyBase Object Reference"))
  (`self.DefaultAttack`)
  (return self))

(fn `AI_GetIdealRange`
  (returns (AttackRadius :type "Float (double-precision)") (DefendRadius :type "Float (double-precision)"))
  (return 150.0 400.0))

(fn `AI_GetPatrolRoute`
  (returns (PatrolRoute :type "/Game/AI/BP_PatrolRoute Object Reference"))
  (return (`self.PatrolRoute`)))

(fn `AI_IsWieldingSword`
  (returns (IsWieldingSword :type Boolean))
  (return (`self.IsWieldingSword`)))

(fn `AI_SetMovementSpeed`
  (params (MovementMode :type "/Game/AI/Enums/E_AIMovementModes Enum" :default "NewEnumerator0"))
  (returns (Speed :type "Float (double-precision)"))
  (bind _output_get (set `CharacterMovementComponent.MaxWalkSpeed` (select `/Game/AI/Enums/E_AIMovementModes` MovementMode :`NewEnumerator1` 100.0 :`NewEnumerator2` 300.0 :`NewEnumerator3` 500.0 :!type "Float (single-precision)") (`self.CharacterMovement`)))
  (return _output_get))

(fn `AI_SheatSword`
  (returns (BP_EnemyBase :type "/Game/Blueprints/Enemies/BP_EnemyBase Object Reference"))
  (`self.SheathSword`)
  (return self))

(fn `AI_WieldSword`
  (returns (BP_EnemyBase :type "/Game/Blueprints/Enemies/BP_EnemyBase Object Reference"))
  (`self.WieldSword`)
  (return self))

(fn `Backstab`
  (returns (BackStabberLoc :type "Vector Structure") (BackStabberRot :type "Rotator Structure"))
  (`self.DieAnimation`)
  (return (`SceneComponent.K2_GetComponentLocation` (`self.BackStabRef`)) (`self.K2_GetActorRotation`)))

(fn `DeadSettings`
  (`PrimitiveComponent.SetSimulatePhysics` (`self.Mesh`) true)
  (`self.Ragdoll`)
  (`PrimitiveComponent.SetCollisionEnabled` (`self.CapsuleComponent`) "QueryOnly")
  (`PrimitiveComponent.SetCollisionEnabled` (`self.BackStabCollision`) "NoCollision")
  (`self.SetLifeSpanAfterDied`))

(fn `UserConstructionScript`)