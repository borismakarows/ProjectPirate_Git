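; Melee enemy Blueprint that provides AI-callable attack, equip weapon and unequip weapon actions.
; AI wrapper functions trigger montage-driven events and return self, with end notifications called on montage completion or interruption.
; Equip plays the wielding montage in reverse, then after a short delay spawns a data-table-configured Morningstar on the right-hand socket.
; Unequip plays a sheathing montage and destroys the weapon actor after a timed delay.
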(event `DefaultAttack`
  ;[0.8229 0 0.006893 0.5] AI Default Attack
  (`|PlayMontage` (`self.Mesh`) "/Game/Animations/Maris/Attack/Attack2_Montage.Attack2_Montage"
    (:`OnCompleted`
      _)
    (:`OnInterrupted`
      _))
  (`self.OnAttackEnd`))

(event `EquipWeapon`
  ;[0.2314 0.4688 0 0.5] EquipWeapon
  (`|PlayMontage` (`self.Mesh`) "/Game/Animations/Enemy/Armed/WieldingSword_Montage.WieldingSword_Montage" -1.0 1.25
    (:`then`
      (`KismetSystemLibrary.Delay` 0.2)
      (bind _returnvalue (`|SpawnActorFromClass` "/Game/InventorySystem/Swords/BP_Morningstar.BP_Morningstar_C" (`self.GetTransform`) "Undefined" "MultiplyWithRoot" null (make `/Game/InventorySystem/S_Slots` (make `DataTableRowHandle` "/Game/InventorySystem/DB_Items.DB_Items" (`self.WeaponItemRowName`))) null))
      (bind _output_get (set `self.WeaponActor` _returnvalue))
      (`self.K2_AttachToComponent` _output_get (`self.Mesh`) "Weaponhand_r" "SnapToTarget" "SnapToTarget" "SnapToTarget" true)
      (set `self.IsEquippedWeapon` true))
    (:`OnCompleted`
      (`self.OnEquipWeaponEnd` :!label _label))
    (:`OnInterrupted`
      (goto _label))))

(event `UnequipWeapon`
  ;[0 0.9844 0.8481 0.5] UnEquipWeapon
  (`|PlayMontage` (`self.Mesh`) "/Game/Animations/Enemy/Armed/SheathingSword_Montage.SheathingSword_Montage"
    (:`then`
      (`KismetSystemLibrary.Delay` 1.05)
      (`self.K2_DestroyActor` (`self.WeaponActor`)))
    (:`OnCompleted`
      (`self.OnUnEquipWeaponEnd` :!label _label_2)
      (set `self.IsEquippedWeapon` false))
    (:`OnInterrupted`
      (goto _label_2))))

(fn `AI_Attack`
  (returns (BP_EnemyBase :type "/Game/Blueprints/Enemies/BP_EnemyBase Object Reference"))
  (`self.DefaultAttack`)
  (return self))

(fn `AI_EquipWeapon`
  (returns (BP_EnemyBase :type "/Game/Blueprints/Enemies/BP_EnemyBase Object Reference"))
  (`self.EquipWeapon`)
  (return self))

(fn `AI_UnEquipWeapon`
  (returns (BP_EnemyBase :type "/Game/Blueprints/Enemies/BP_EnemyBase Object Reference"))
  (`self.UnequipWeapon`)
  (return self))

(fn `UserConstructionScript`
  (`parent.UserConstructionScript`))