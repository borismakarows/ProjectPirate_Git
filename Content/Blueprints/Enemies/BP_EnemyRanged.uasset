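; Ranged enemy that equips a flintlock pistol and shoots its attack target, overriding AI functions for attack, equip, ideal range and movement speed.
; Equipping turns toward the controller's attack target, plays a montage and, after a delay, spawns the pistol on a hand socket.
; Attacks play a shoot montage, then line-trace from weapon to target so the damage system component hurts the first non-team hit.
; Montage completion or interruption ends either action.
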(event `Attack`
  (params (AttackTarget :type "Actor Object Reference"))
  ; Attack
  (`self.WeaponActor`
    (:`then`
      (`|PlayMontage` (`self.Mesh`) "/Game/Animations/Enemy/Ranged/ShootPistol_Montage.ShootPistol_Montage"
        (:`then`
          (`KismetSystemLibrary.Delay` 0.1)
          (bind (_outhits _returnvalue) (`KismetSystemLibrary.LineTraceMulti` (`self.K2_GetActorLocation` (`self.WeaponActor`)) (`self.K2_GetActorLocation` AttackTarget) "TraceTypeQuery1"))
          (if _returnvalue
            (`/Game/Blueprints/Enemies/BPC_AIDamageSystem.DamageFirstNonTeamMembers` (`self.BPC_AIDamageSystem`) _outhits (make `/Game/Blueprints/DamageSystem/S_DamageInfo` 10.0 "NewEnumerator2" "NewEnumerator0" false false false false self))))
        (:`OnCompleted`
          (`self.AI_AttackEnd` AttackTarget :!label _label))
        (:`OnInterrupted`
          (goto _label))))
    (:`else`)))

(event `self.EquipWeapon`
  ; Equip Weapon
  (`self.TurnToPlayer`)
  (`|PlayMontage` (`self.Mesh`) "/Game/Animations/Enemy/Ranged/EquipPistol_Montage.EquipPistol_Montage" 1.75
    (:`then`
      (`KismetSystemLibrary.Delay` 1.25)
      (bind _returnvalue (`|SpawnActorFromClass` "/Game/Blueprints/InventorySystem/Guns/BP_Flintlock.BP_Flintlock_C" (`self.GetTransform`) "Undefined" "MultiplyWithRoot" null (make `/Game/Blueprints/InventorySystem/S_Slots` (make `DataTableRowHandle` "/Game/Blueprints/InventorySystem/DB_Items.DB_Items" (`self.WeaponItemRowName`))) null))
      (bind _output_get (set `self.WeaponActor` _returnvalue))
      (`self.K2_AttachToComponent` _output_get (`self.Mesh`) "hand_l_Pistol" "SnapToTarget" "SnapToTarget" "SnapToTarget" true))
    (:`OnCompleted`
      (set `self.IsEquippedWeapon` true :!label _label_2)
      (`self.OnEquipWeaponEnd`))
    (:`OnInterrupted`
      (goto _label_2))))

(fn `AI_Attack`
  (params (AttackTarget :type "Actor Object Reference"))
  (set `self.IsAttacking?` true)
  (`self.Attack` AttackTarget)
  (return))

(fn `AI_AttackStart`
  (params (AttackTarget :type "Actor Object Reference") (TokensNeeded :type Integer))
  (returns (Success :type Boolean))
  (bind _success (`parent.AI_AttackStart` AttackTarget TokensNeeded))
  (return _success))

(fn `AI_EquipWeapon`
  (returns (BP_EnemyBase :type "/Game/Blueprints/Enemies/BP_EnemyBase Object Reference"))
  (`self.EquipWeapon`)
  (return self))

(fn `AI_GetIdealRange`
  (returns (AttackRadius :type "Float (double-precision)") (DefendRadius :type "Float (double-precision)"))
  (return 600.0 600.0))

(fn `AI_SetMovementSpeed`
  (params (MovementMode :type "/Game/Blueprints/AI/Enums/E_AIMovementModes Enum" :default "NewEnumerator0"))
  (returns (Speed :type "Float (double-precision)"))
  (set `CharacterMovementComponent.MaxWalkSpeed` (select `/Game/Blueprints/AI/Enums/E_AIMovementModes` MovementMode :`NewEnumerator1` 100.0 :`NewEnumerator2` 300.0 :`NewEnumerator3` 500.0 :!type "Float (single-precision)") (`self.CharacterMovement`))
  (return 0.0))

(fn `TurnToPlayer`
  (bind _attacktarget (message `/Game/Blueprints/AI/BPI_AIController.GetAttackTarget` (`AIBlueprintHelperLibrary.GetAIController` self)))
  (`/Engine/EditorBlueprintResources/StandardMacros.IsValid` _attacktarget
    (:`Is Valid`
      (`self.K2_AddActorWorldRotation` (`KismetMathLibrary.FindLookAtRotation` (`self.K2_GetActorLocation`) (`self.K2_GetActorLocation` _attacktarget))))))

(fn `UserConstructionScript`
  (`parent.UserConstructionScript`))