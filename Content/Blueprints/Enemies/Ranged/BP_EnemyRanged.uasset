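; Ranged enemy Blueprint that fights with a flintlock pistol, spawned from the item table and attached to the mesh on BeginPlay.
; Equip and unequip play one montage forward or reversed, using notifies to switch sockets and toggling interruptibility.
; Every AI attack type routes to PistolShot, whose montage notify fires a sphere trace through the AI damage component, damaging non-team targets.
; AI overrides supply ideal range, movement speeds and patrol route.
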(event `self.ReceiveBeginPlay`
  (`parent.ReceiveBeginPlay`)
  ;[0.04801 0.05208 0.05083] Spawn Weapon
  (bind _returnvalue (`|SpawnActorFromClass` "/Game/Blueprints/InventorySystem/Guns/BP_Flintlock.BP_Flintlock_C" (`self.GetTransform`) "Undefined" "MultiplyWithRoot" null (make `/Game/Blueprints/InventorySystem/S_Slots` (make `DataTableRowHandle` "/Game/Blueprints/InventorySystem/DB_Items.DB_Items" (`self.WeaponItemRowName`))) false 0.0 0.0 null))
  (bind _output_get (set `self.WeaponActor` _returnvalue))
  (`self.K2_AttachToComponent` _output_get (`self.Mesh`) "GunSocket_r" "SnapToTarget" "SnapToTarget" "SnapToTarget" true)
  (`PrimitiveComponent.SetCollisionEnabled` (`/Game/Blueprints/InventorySystem/BP_MasterItem.Mesh` _output_get) "NoCollision")
  (set `/Game/Blueprints/Maris/Components/BPC_StatManager.IsInterruptible` true (`self.BPC_Stats`)))

(event `UnEquip Weapon`
  ;[1 0.6731 0.002336 0.5] Unequip
  (bind _notifyname (`|PlayMontage` (`self.Mesh`) "/Game/Assets/Enemies/Animation/Ranged/EquipPistol_Montage.EquipPistol_Montage" -1.75)
    (:`OnCompleted`
      (`self.OnUnEquipWeaponEnd` :!label _label)
      (set `self.IsEquippedWeapon` false)
      (set `/Game/Blueprints/Maris/Components/BPC_StatManager.IsInterruptible` true (`self.BPC_Stats`)))
    (:`OnInterrupted`
      (goto _label))
    (:`OnNotifyBegin`
      (switch `name` _notifyname
        (:`Equip`
          (`self.K2_AttachToComponent` (`self.WeaponActor`) (`self.Mesh`) "SwordSheat_r" "SnapToTarget" "SnapToTarget" "SnapToTarget" true))))))

(event `self.EquipWeapon`
  ;[1 0.7939 0 0.5] Equip
  (set `/Game/Blueprints/Maris/Components/BPC_StatManager.IsInterruptible` false (`self.BPC_Stats`))
  (bind _notifyname (`|PlayMontage` (`self.Mesh`) "/Game/Assets/Enemies/Animation/Ranged/EquipPistol_Montage.EquipPistol_Montage" 2.0)
    (:`OnCompleted`
      (set `self.IsEquippedWeapon` true :!label _label_2)
      (set `/Game/Blueprints/Maris/Components/BPC_StatManager.IsInterruptible` true (`self.BPC_Stats`))
      (`self.OnEquipWeaponEnd`))
    (:`OnInterrupted`
      (goto _label_2))
    (:`OnNotifyBegin`
      (switch `name` _notifyname
        (:`Equip`
          (`self.K2_AttachToComponent` (`self.WeaponActor`) (`self.Mesh`) "hand_l_Pistol" "SnapToTarget" "SnapToTarget" "SnapToTarget" true))))))

(event `PistolShot`
  (params (AttackTarget :type "Actor Object Reference"))
  ; Attack
  (`self.WeaponActor`
    (:`then`
      (bind _notifyname (`|PlayMontage` (`self.Mesh`) "/Game/Assets/Enemies/Animation/Ranged/ShootPistol_Montage.ShootPistol_Montage")
        (:`then`
          (set `/Game/Blueprints/Maris/Components/BPC_StatManager.IsInterruptible` true (`self.BPC_Stats`)))
        (:`OnCompleted`
          (`self.AI_AttackEnd` AttackTarget :!label _label_3))
        (:`OnInterrupted`
          (goto _label_3))
        (:`OnNotifyBegin`
          (switch `name` _notifyname
            (:`Shoot`
              (bind (_hitresults _hit_) (`/Game/Blueprints/Enemies/BPC_AIDamageSystem.MultiSphereTrace` (`self.BPC_AIDamageSystem`) (`self.Attack Range`) AttackTarget))
              (if _hit_
                (`/Game/Blueprints/Enemies/BPC_AIDamageSystem.DamageFirstNonTeamMembers` (`self.BPC_AIDamageSystem`) _hitresults (make `/Game/Blueprints/DamageSystem/S_DamageInfo` 10.0 "NewEnumerator2" "NewEnumerator0" false false false false self))))))))
    (:`else`)))

(event `/Game/Blueprints/AI/BPI_EnemyAI.AI_Attacks`
  (params (AttackTarget :type "Actor Object Reference") (AttackTypes :type "/Game/Blueprints/Enemies/E_AttackTypes Enum" :default "NewEnumerator0"))
  (switch `/Game/Blueprints/Enemies/E_AttackTypes` AttackTypes
    (:`NewEnumerator0`
      (`self.PistolShot` AttackTarget))
    (:`NewEnumerator1`
      (`self.PistolShot` AttackTarget))
    (:`NewEnumerator2`
      (`self.PistolShot` AttackTarget :!label _label_4))
    (:`NewEnumerator3`
      (goto _label_4))))

(fn `AI_AttackStart`
  (params (AttackTarget :type "Actor Object Reference") (TokensNeeded :type Integer))
  (returns (Success :type Boolean))
  (bind _success (`parent.AI_AttackStart` AttackTarget TokensNeeded))
  (return _success))

(fn `AI_EquipWeapon`
  (returns (BP_EnemyBase :type "/Game/Blueprints/Enemies/BP_EnemyBase Object Reference"))
  (`self.EquipWeapon`)
  (return self))

(fn `AI_GetIdealRange`
  (returns (AttackRadius :type "Float (double-precision)") (DefendRadius :type "Float (double-precision)"))
  (return 600.0 600.0))

(fn `AI_GetPatrolRoute`
  (returns (PatrolRoute :type "/Game/Blueprints/AI/BP_PatrolRoute Object Reference"))
  (return (`self.PatrolRoute`)))

(fn `AI_SetMovementSpeed`
  (params (MovementMode :type "/Game/Blueprints/AI/Enums/E_AIMovementModes Enum" :default "NewEnumerator0"))
  (returns (Speed :type "Float (double-precision)"))
  (bind _output_get (set `CharacterMovementComponent.MaxWalkSpeed` (select `/Game/Blueprints/AI/Enums/E_AIMovementModes` MovementMode :`NewEnumerator1` 100.0 :`NewEnumerator2` 300.0 :`NewEnumerator3` 500.0 :!type "Float (single-precision)") (`self.CharacterMovement`)))
  (return _output_get))

(fn `TurnToPlayer`
  (bind _attacktarget (message `/Game/Blueprints/AI/BPI_AIController.GetAttackTarget` (`AIBlueprintHelperLibrary.GetAIController` self)))
  (`/Engine/EditorBlueprintResources/StandardMacros.IsValid` _attacktarget
    (:`Is Valid`
      (`self.K2_AddActorWorldRotation` (`KismetMathLibrary.FindLookAtRotation` (`self.K2_GetActorLocation`) (`self.K2_GetActorLocation` _attacktarget))))))

(fn `UserConstructionScript`
  (`parent.UserConstructionScript`))