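; Melee enemy character that spawns a morningstar at a back socket, equips and sheathes it via montages, and exposes AI functions for ranges and patrol route.
; AI attacks branch by type into slash, jump or heavy montages, whose notifies run sphere traces that damage non-team members.
; The jump attack launches along an arc toward the target's predicted position.
; Timed blocking plays a reaction montage when hit, then ends.
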(event `self.ReceiveBeginPlay`
  (`parent.ReceiveBeginPlay`)
  ;[0.04801 0.05208 0.05083] Spawn Weapon and Attach
  (bind _returnvalue (`|SpawnActorFromClass` "/Game/Blueprints/InventorySystem/Swords/BP_Morningstar.BP_Morningstar_C" (`self.GetTransform`) "Undefined" "MultiplyWithRoot" null (make `/Game/Blueprints/InventorySystem/S_Slots` (make `DataTableRowHandle` "/Game/Blueprints/InventorySystem/DB_Items.DB_Items" (`self.WeaponItemRowName`))) false 0.0 1.0 null))
  (bind _output_get (set `self.WeaponActor` _returnvalue))
  (`self.K2_AttachToComponent` _output_get (`self.Mesh`) "SwordSheat_r" "SnapToTarget" "SnapToTarget" "SnapToTarget" true)
  (`PrimitiveComponent.SetCollisionResponseToChannel` (`/Game/Blueprints/InventorySystem/BP_MasterItem.Mesh` _output_get) "ECC_GameTraceChannel5" "ECR_Ignore"))

(event `EquipWeapon`
  ;[0.2314 0.4688 0 0.5] EquipWeapon
  (`MovementComponent.StopMovementImmediately` (`self.CharacterMovement`))
  (bind _notifyname (`|PlayMontage` (`self.Mesh`) "/Game/Assets/Enemy/Animation/Armed/WieldingSword_Montage.WieldingSword_Montage" -1.0 1.25)
    (:`OnCompleted`
      (`self.OnEquipWeaponEnd` :!label _label)
      (set `self.IsEquippedWeapon` true))
    (:`OnInterrupted`
      (goto _label))
    (:`OnNotifyBegin`
      (switch `name` _notifyname
        (:`Equip`
          (`self.K2_AttachToComponent` (`self.WeaponActor`) (`self.Mesh`) "SwordHand_r" "SnapToTarget" "SnapToTarget" "SnapToTarget" true))))))

(event `UnequipWeapon`
  ;[0 0.9844 0.8481 0.5] UnEquipWeapon
  (bind _notifyname (`|PlayMontage` (`self.Mesh`) "/Game/Assets/Enemy/Animation/Armed/SheathingSword_Montage.SheathingSword_Montage")
    (:`OnCompleted`
      (`self.OnUnEquipWeaponEnd` :!label _label_2)
      (set `self.IsEquippedWeapon` false))
    (:`OnInterrupted`
      (goto _label_2))
    (:`OnNotifyBegin`
      (switch `name` _notifyname
        (:`Equip`
          (`self.K2_AttachToComponent` (`self.WeaponActor`) (`self.Mesh`) "SwordHand_r" "SnapToTarget" "SnapToTarget" "SnapToTarget" true))))))

(event `StartBlock`
  ;[0.05725 0 1 0.5] EnemyBlock
  (if (`self.IsEquippedWeapon`)
    (`KismetSystemLibrary.K2_ClearAndInvalidateTimerHandle` (`self.HoldBlockTimer`))
    (`MovementComponent.StopMovementImmediately` (`self.CharacterMovement`))
    (set `/Game/Blueprints/Maris/BPC_Stats.IsBlocking` true (`self.BPC_Stats`))
    (set `self.GuardState` "NewEnumerator2")
    (bind _returnvalue (`KismetSystemLibrary.K2_SetTimerDelegate` (`|CreateDelegate` :!event `EndBlock`) 1.0))
    (set `self.HoldBlockTimer` _returnvalue)))

(event `/Game/Blueprints/AI/BPI_EnemyAI.AI_Attacks`
  (params (AttackTarget :type "Actor Object Reference") (AttackTypes :type "/Game/Blueprints/Enemies/E_AttackTypes Enum" :default "NewEnumerator0"))
  ;[0.8229 0 0.006893 0.5] Attack
  (`parent.AI_Attacks` AttackTarget AttackTypes)
  (switch `/Game/Blueprints/Enemies/E_AttackTypes` AttackTypes
    (:`NewEnumerator0`
      (`self.SwordAttack` AttackTarget))
    (:`NewEnumerator1`
      (`self.SwordAttack` AttackTarget))
    (:`NewEnumerator2`
      (`self.JumpAttack` AttackTarget))
    (:`NewEnumerator3`
      (`self.HeavyAttack` AttackTarget))))

(event `self.BPC_Stats.OnBlocked`
  (params (CanBeParried :type Boolean) (Damage :type "Float (double-precision)") (DamageCauser :type "Actor Object Reference"))
  ;[0.05725 0 1 0.5] EnemyBlock
  (set `self.GuardState` "NewEnumerator3")
  (`KismetSystemLibrary.K2_ClearAndInvalidateTimerHandle` (`self.HoldBlockTimer`))
  (`|PlayMontage` (`self.Mesh`) "/Game/Assets/Enemy/Animation/Guard/StandingBlockReactLarge_UE_Montage.StandingBlockReactLarge_UE_Montage"
    (:`OnCompleted`
      _)
    (:`OnInterrupted`
      _))
  (`self.EndBlock`))

(event `EndBlock`
  ;[0.05725 0 1 0.5] EnemyBlock
  (set `/Game/Blueprints/Maris/BPC_Stats.IsBlocking` false (`self.BPC_Stats`))
  (set `self.GuardState` "NewEnumerator0")
  (`self.OnBlockEnd`))

(event `SwordAttack`
  (params (AttackTarget :type "Actor Object Reference"))
  (bind _bpc_stats (`self.BPC_Stats`))
  ;[0.8229 0 0.006893 0.5] Attack
  ;; SwordSlash
  (bind _notifyname (`|PlayMontage` (`self.Mesh`) "/Game/Assets/Maris/Animation/Attack/Attack2_Montage.Attack2_Montage")
    (:`OnCompleted`
      (`self.AI_AttackEnd` AttackTarget :!label _label_3)
      (set `/Game/Blueprints/Maris/BPC_Stats.IsInterruptible` true _bpc_stats))
    (:`OnInterrupted`
      (goto _label_3))
    (:`OnNotifyBegin`
      (switch `name` _notifyname
        (:`Hit`
          (set `/Game/Blueprints/Maris/BPC_Stats.IsInterruptible` false _bpc_stats)
          (bind (_hitresults _hit_) (`/Game/Blueprints/Enemies/BPC_AIDamageSystem.MultiSphereTrace` (`self.BPC_AIDamageSystem`) (`self.Attack Range`) null))
          (if _hit_
            (`/Game/Blueprints/Enemies/BPC_AIDamageSystem.DamageAllNonTeamMembers` (`self.BPC_AIDamageSystem`) _hitresults (make `/Game/Blueprints/DamageSystem/S_DamageInfo` 15.0 "NewEnumerator1" "NewEnumerator0" false true false false self))))))))

(event `JumpAttack`
  (params (AttackTarget :type "Actor Object Reference"))
  (bind _bpc_stats (`self.BPC_Stats`))
  ;[0.8229 0 0.006893 0.5] Attack
  ;; JumpAttack
  (bind _notifyname (`|PlayMontage` (`self.Mesh`) "/Game/Assets/Enemy/Animation/Specials/JumpAttack_Montage.JumpAttack_Montage")
    (:`OnCompleted`
      (`self.AI_AttackEnd` AttackTarget :!label _label_4)
      (set `/Game/Blueprints/Maris/BPC_Stats.IsInterruptible` true _bpc_stats))
    (:`OnInterrupted`
      (goto _label_4))
    (:`OnNotifyBegin`
      (switch `name` _notifyname
        (:`Jump`
          (set `/Game/Blueprints/Maris/BPC_Stats.IsInterruptible` false _bpc_stats)
          (`self.JumpToAttackTarget` AttackTarget))
        (:`Attack`
          (bind (_hitresults _hit_) (`/Game/Blueprints/Enemies/BPC_AIDamageSystem.MultiSphereTrace` (`self.BPC_AIDamageSystem`) 160.0 AttackTarget))
          (if _hit_
            (`/Game/Blueprints/Enemies/BPC_AIDamageSystem.DamageFirstNonTeamMembers` (`self.BPC_AIDamageSystem`) _hitresults (make `/Game/Blueprints/DamageSystem/S_DamageInfo` 20.0 "NewEnumerator1" "NewEnumerator1" false true true false self))))))))

(event `JumpToAttackTarget`
  (params (AttackTarget :type "Actor Object Reference"))
  ;[0.8229 0 0.006893 0.5] Attack
  ;;[0.04801 0.05208 0.05083] Jump Calculation
  (bind _location (`self.CalculateFutureActorLocation` AttackTarget 0.5))
  (bind _outlaunchvelocity (`GameplayStatics.SuggestProjectileVelocity_CustomArc` (`self.K2_GetActorLocation`) (`KismetMathLibrary.MakeVector` (.x _location) (.y _location) (+ (.z _location) 20.0))))
  (`self.LaunchCharacter` _outlaunchvelocity true true)
  (add `self.LandedDelegate` (delegate `Landed_StopMove`)))

(event `Landed_StopMove` :!signature `self.LandedDelegate`
  (params (Hit :type "HitResult Structure (by ref)"))
  ;[0.8229 0 0.006893 0.5] Attack
  ;;[0.04801 0.05208 0.05083] Jump Calculation
  (remove `self.LandedDelegate` (delegate `Landed_StopMove`))
  (`MovementComponent.StopMovementImmediately` (`self.CharacterMovement`)))

(event `HeavyAttack`
  (params (AttackTarget :type "Actor Object Reference"))
  ;[0.8229 0 0.006893 0.5] Attack
  ;; Heavy Attack
  (bind _notifyname (`|PlayMontage` (`self.Mesh`) "/Game/Assets/Enemy/Animation/Specials/HeavyAttack_Montage.HeavyAttack_Montage")
    (:`OnCompleted`
      (`self.AI_AttackEnd` AttackTarget :!label _label_5)
      (set `/Game/Blueprints/Maris/BPC_Stats.IsInterruptible` true (`self.BPC_Stats`)))
    (:`OnInterrupted`
      (goto _label_5))
    (:`OnNotifyBegin`
      (switch `name` _notifyname
        (:`Hit`
          (set `/Game/Blueprints/Maris/BPC_Stats.IsInterruptible` false (`self.BPC_Stats`))
          (bind (_hitresults _hit_) (`/Game/Blueprints/Enemies/BPC_AIDamageSystem.MultiSphereTrace` (`self.BPC_AIDamageSystem`) (+ (`self.Attack Range`) 10.0) AttackTarget))
          (if _hit_
            (`/Game/Blueprints/Enemies/BPC_AIDamageSystem.DamageAllNonTeamMembers` (`self.BPC_AIDamageSystem`) _hitresults (make `/Game/Blueprints/DamageSystem/S_DamageInfo` 30.0 "NewEnumerator1" "NewEnumerator2" false false false true self))))
        (:`BackHit`
          (bind (_hitresults_2 _hit__2) (`/Game/Blueprints/Enemies/BPC_AIDamageSystem.MultiSphereTrace` (`self.BPC_AIDamageSystem`) (- (`self.Attack Range`) 10.0) AttackTarget))
          (if _hit__2
            (`/Game/Blueprints/Enemies/BPC_AIDamageSystem.DamageFirstNonTeamMembers` (`self.BPC_AIDamageSystem`) _hitresults_2 (make `/Game/Blueprints/DamageSystem/S_DamageInfo` 20.0 "NewEnumerator1" "NewEnumerator1" false true true false self))))))))

(fn `AI_AttackStart`
  (params (AttackTarget :type "Actor Object Reference") (TokensNeeded :type Integer))
  (returns (Success :type Boolean))
  (bind _success (`parent.AI_AttackStart` AttackTarget TokensNeeded))
  (return _success))

(fn `AI_EquipWeapon`
  (returns (BP_EnemyBase :type "/Game/Blueprints/Enemies/BP_EnemyBase Object Reference"))
  (`self.EquipWeapon`)
  (return self))

(fn `AI_GetIdealRange`
  (returns (AttackRadius :type "Float (double-precision)") (DefendRadius :type "Float (double-precision)"))
  (return 160.0 300.0))

(fn `AI_GetPatrolRoute`
  (returns (PatrolRoute :type "/Game/Blueprints/AI/BP_PatrolRoute Object Reference"))
  (return (`self.PatrolRoute`)))

(fn `AI_UnEquipWeapon`
  (returns (BP_EnemyBase :type "/Game/Blueprints/Enemies/BP_EnemyBase Object Reference"))
  (`self.UnequipWeapon`)
  (return self))

(fn `CalculateFutureActorLocation`
  (params (Actor :type "Actor Object Reference") (Time :type "Float (double-precision)"))
  (returns (Location :type "Vector Structure"))
  (bind (_returnvalue_x _returnvalue_y) (`KismetMathLibrary.BreakVector` (`self.GetVelocity` Actor)))
  (return (+ (`self.K2_GetActorLocation` Actor) (* (`KismetMathLibrary.MakeVector` _returnvalue_x _returnvalue_y) Time))))

(fn `GetHealthValues`
  (returns (MaxHealth :type "Float (double-precision)") (CurrentHealth :type "Float (double-precision)") (`IsDead?` :type Boolean))
  (bind _bpc_stats (`self.BPC_Stats`))
  (return (`/Game/Blueprints/Maris/BPC_Stats.MaxHealth` _bpc_stats) (`/Game/Blueprints/Maris/BPC_Stats.CurrentHealth` _bpc_stats) (`/Game/Blueprints/Maris/BPC_Stats.IsDead` _bpc_stats)))

(fn `TakeDamage`
  (params (DamageInfo :type "/Game/Blueprints/DamageSystem/S_DamageInfo Structure"))
  (returns (WasDamaged :type Boolean))
  (bind _wasdamaged (`parent.TakeDamage` DamageInfo))
  (return _wasdamaged))

(fn `UserConstructionScript`
  (`parent.UserConstructionScript`))