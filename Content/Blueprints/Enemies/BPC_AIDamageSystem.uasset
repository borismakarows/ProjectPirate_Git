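; AI damage component that traces enemy attacks and applies damage to actors outside the owner's team.
; MultiSphereTrace sweeps a small debug-drawn sphere from the owner to the target, or straight forward at attack range if the target is invalid or out of range.
; Damage functions compare team numbers via messages, then send TakeDamageMessage to either the first non-teammate hit or each unique one.
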(fn `DamageAllNonTeamMembers`
  (params (Hits :type "Array of HitResult Structure") (DamageInfo :type "/Game/Blueprints/DamageSystem/S_DamageInfo Structure"))
  (returns (DamagedActors :type "Array of Actor Object Reference"))
  (locals (ActorDamageSoFar :type "Array of Actor Object Reference"))
  (bind _actordamagesofar (`local.ActorDamageSoFar`))
  (for _array_element Hits
    (bind (_bblockinghit _binitialoverlap _time _distance _location _impactpoint _normal _impactnormal _physmat _hitactor) (`GameplayStatics.BreakHitResult` _array_element))
    (bind _sameteam (`self.OnSameTeam` _hitactor))
    (if (and (not _sameteam) (not (`KismetArrayLibrary.Array_Contains` _actordamagesofar _hitactor)))
      (message `/Game/Blueprints/DamageSystem/BPI_StatManagement.TakeDamage` _hitactor DamageInfo)
      (`KismetArrayLibrary.Array_AddUnique` (`local.ActorDamageSoFar`) _hitactor)))
  (return _actordamagesofar))

(fn `DamageFirstNonTeamMembers`
  (params (Hits :type "Array of HitResult Structure") (`Damage Info` :type "/Game/Blueprints/DamageSystem/S_DamageInfo Structure"))
  (returns (DamagedActor :type "Actor Object Reference"))
  (for _array_element Hits
    (bind (_bblockinghit _binitialoverlap _time _distance _location _impactpoint _normal _impactnormal _physmat _hitactor) (`GameplayStatics.BreakHitResult` _array_element))
    (bind _sameteam (`self.OnSameTeam` _hitactor))
    (if (not _sameteam)
      (message `/Game/Blueprints/DamageSystem/BPI_StatManagement.TakeDamage` _hitactor `Damage Info`)
      (`|ExecutionSequence`
        (:`then_0`
          (break))
        (:`then_1`
          (return _hitactor))))))

(fn `MultiSphereTrace`
  (params (AttackRange :type "Float (double-precision)") (AttackTarget :type "Actor Object Reference"))
  (returns (HitResults :type "Array of HitResult Structure") (`Hit?` :type Boolean))
  (locals (EndLoc :type "Vector Structure" :default (0.0 0.0 0.0)))
  (bind _returnvalue (`self.GetOwner`))
  (`local.AttackTarget`
    (:`then`
      (set `local.EndLoc` (`Actor.K2_GetActorLocation` (`local.AttackTarget`)))
      (if (not (>= (`local.AttackRange`) (`KismetMathLibrary.Vector_Distance2D` (`Actor.K2_GetActorLocation` (`self.GetOwner`)) (`local.EndLoc`))))
        (set `local.EndLoc` (+ (`Actor.K2_GetActorLocation` _returnvalue) (* (`Actor.GetActorForwardVector` _returnvalue) (`local.AttackRange`))) :!label _label)))
    (:`else`
      (goto _label)))
  (bind (_outhits _returnvalue_2) (`KismetSystemLibrary.SphereTraceMulti` (`Actor.K2_GetActorLocation` (`self.GetOwner`)) (`local.EndLoc`) 8.0 "TraceTypeQuery1" false (`|MakeArray` (`self.GetOwner`)) "ForDuration"))
  (return _outhits _returnvalue_2))

(fn `OnSameTeam`
  (params (Actor :type "Actor Object Reference"))
  (returns (SameTeam :type Boolean))
  (bind _teamnumber (message `/Game/Blueprints/DamageSystem/BPI_StatManagement.GetTeamNumber` Actor))
  (bind _teamnumber_2 (message `/Game/Blueprints/DamageSystem/BPI_StatManagement.GetTeamNumber` (`self.GetOwner`)))
  (return (== _teamnumber_2 _teamnumber)))