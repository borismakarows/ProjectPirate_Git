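; Rogue enemy character that fights with a dagger up close and a thrown dagger at long range, drawing its weapon first if sheathed.
; AI interface functions supply speeds, ranges and patrol route, and trigger equipping, which reuses the sheathing montage in reverse.
; Montage notifies drive socket swaps, the parryable melee sphere trace with its interruptible window, and spawning of zero-gravity BP_MasterItem projectiles that damage on impact.
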(event `self.ReceiveBeginPlay`
  (`parent.ReceiveBeginPlay`)
  ;[0.04801 0.05208 0.05083] Spawn Sword At the Beginning
  (bind _returnvalue (`|SpawnActorFromClass` "/Game/Blueprints/InventorySystem/BP_MasterItem.BP_MasterItem_C" (`self.GetTransform`) "AlwaysSpawn" "MultiplyWithRoot" null (make `/Game/Blueprints/InventorySystem/S_Slots` (make `DataTableRowHandle` "/Game/Blueprints/InventorySystem/DB_Items.DB_Items" (`self.WeaponItemRowName`))) false 0.0 1.0 null))
  (bind _output_get (set `self.WeaponActor` _returnvalue))
  (`PrimitiveComponent.SetCollisionEnabled` (`/Game/Blueprints/InventorySystem/BP_MasterItem.Mesh` _output_get) "NoCollision")
  (`self.K2_AttachToComponent` _output_get (`self.Mesh`) "SwordSheat_r" "SnapToTarget" "SnapToTarget" "SnapToTarget" true)
  (set `/Game/Blueprints/Maris/Components/BPC_StatManager.IsInterruptible` true (`self.BPC_Stats`)))

(event `EquipWeapon`
  ;[0.776 0 0 0.5] Equip Weapon
  (`self.WeaponActor`
    (:`then`
      (set `/Game/Blueprints/Maris/Components/BPC_StatManager.IsInterruptible` false (`self.BPC_Stats`))
      (`MovementComponent.StopMovementImmediately` (`self.CharacterMovement`))
      (bind _notifyname (`|PlayMontage` (`self.Mesh`) "/Game/Assets/Enemies/Animation/Armed/SheathingSword_Montage.SheathingSword_Montage" -1.0 1.25)
        (:`OnCompleted`
          (`self.OnEquipWeaponEnd` :!label _label)
          (set `/Game/Blueprints/Maris/Components/BPC_StatManager.IsInterruptible` true (`self.BPC_Stats`))
          (set `self.IsEquippedWeapon` true))
        (:`OnInterrupted`
          (goto _label))
        (:`OnNotifyBegin`
          (switch `name` _notifyname
            (:`Equip`
              (`self.K2_AttachToComponent` (`self.WeaponActor`) (`self.Mesh`) "SwordHand_r" "SnapToTarget" "SnapToTarget" "SnapToTarget" true))))))
    (:`else`)))

(event `/Game/Blueprints/AI/BPI_EnemyAI.AI_Attacks`
  (params (AttackTarget :type "Actor Object Reference") (AttackTypes :type "/Game/Blueprints/Enemies/E_AttackTypes Enum" :default "NewEnumerator0"))
  ;[1 0.1067 0] Attack
  (if (`self.IsEquippedWeapon`)
    (switch `/Game/Blueprints/Enemies/E_AttackTypes` AttackTypes
      (:`NewEnumerator0`
        (`self.DaggerAttack` AttackTarget))
      (:`NewEnumerator1`
        (`self.DaggerAttack` AttackTarget))
      (:`NewEnumerator2`
        (`self.SlingAttack` AttackTarget)))
    (else
      (`self.EquipWeapon`))))

(event `DaggerAttack`
  (params (AttackTarget :type "Actor Object Reference"))
  ;[1 0.1067 0] Attack
  ;; Melee
  (set `/Game/Blueprints/Maris/Components/BPC_StatManager.IsInterruptible` false (`self.BPC_Stats`))
  (bind _notifyname (`|PlayMontage` (`self.Mesh`) (`|GetArrayItem` (`self.DaggerAttackMontages`) (`KismetMathLibrary.RandomIntegerInRange` 0 1)))
    (:`OnCompleted`
      (`self.AI_AttackEnd` AttackTarget :!label _label_2)
      (set `/Game/Blueprints/Maris/Components/BPC_StatManager.IsInterruptible` true (`self.BPC_Stats`)))
    (:`OnInterrupted`
      (goto _label_2))
    (:`OnNotifyBegin`
      (switch `name` _notifyname
        (:`ParryWindow`
          (set `/Game/Blueprints/Maris/Components/BPC_StatManager.IsInterruptible` true (`self.BPC_Stats`))
          ;;; Hit Trace
          (bind (_hitresults _hit_) (`/Game/Blueprints/Enemies/BPC_AIDamageSystem.MultiSphereTrace` (`self.BPC_AIDamageSystem`) (`self.AttackRange`) null))
          (if _hit_
            (`/Game/Blueprints/Enemies/BPC_AIDamageSystem.DamageFirstNonTeamMembers` (`self.BPC_AIDamageSystem`) _hitresults (make `/Game/Blueprints/DamageSystem/S_DamageInfo` 5.0 "NewEnumerator1" "NewEnumerator1" false true true false self))))))
    (:`OnNotifyEnd`
      (switch `name` _notifyname
        (:`ParryWindow`
          (set `/Game/Blueprints/Maris/Components/BPC_StatManager.IsInterruptible` false (`self.BPC_Stats`)))))))

(event `UnequipWeapon`
  ;[0 0.7188 0.01068 0.5] Unequip Sword
  (set `/Game/Blueprints/Maris/Components/BPC_StatManager.IsInterruptible` false (`self.BPC_Stats`))
  (bind _notifyname (`|PlayMontage` (`self.Mesh`) "/Game/Assets/Enemies/Animation/Armed/SheathingSword_Montage.SheathingSword_Montage")
    (:`OnCompleted`
      (`self.OnUnEquipWeaponEnd` :!label _label_3)
      (set `self.IsEquippedWeapon` false)
      (set `/Game/Blueprints/Maris/Components/BPC_StatManager.IsInterruptible` true (`self.BPC_Stats`)))
    (:`OnInterrupted`
      (goto _label_3))
    (:`OnNotifyBegin`
      (switch `name` _notifyname
        (:`Equip`
          (`self.K2_AttachToComponent` (`self.WeaponActor`) (`self.Mesh`) "SwordSheat_r" "SnapToTarget" "SnapToTarget" "SnapToTarget" true))))))

(event `SlingAttack`
  (params (AttackTarget :type "Actor Object Reference"))
  ;[1 0.1067 0] Attack
  ;; Sling
  (`SceneComponent.SetVisibility` (`/Game/Blueprints/InventorySystem/BP_MasterItem.Mesh` (`self.WeaponActor`)) false false)
  (bind _notifyname (`|PlayMontage` (`self.Mesh`) "/Game/Assets/Enemies/Animation/Rogue/ThrowSling_Montage.ThrowSling_Montage")
    (:`OnCompleted`
      (`self.AI_AttackEnd` AttackTarget :!label _label_4)
      (`SceneComponent.SetVisibility` (`/Game/Blueprints/InventorySystem/BP_MasterItem.Mesh` (`self.WeaponActor`)) true false)
      (set `/Game/Blueprints/Maris/Components/BPC_StatManager.IsInterruptible` true (`self.BPC_Stats`)))
    (:`OnInterrupted`
      (goto _label_4))
    (:`OnNotifyBegin`
      (switch `name` _notifyname
        (:`Throw`
          (bind _returnvalue (`|SpawnActorFromClass` "/Game/Blueprints/InventorySystem/BP_MasterItem.BP_MasterItem_C" (`KismetMathLibrary.MakeTransform` (`SceneComponent.GetSocketLocation` (`self.Mesh`) "SlingThrowHand_r") (`self.K2_GetActorRotation`)) "AlwaysSpawn" "MultiplyWithRoot" null (make `/Game/Blueprints/InventorySystem/S_Slots` (make `DataTableRowHandle` "/Game/Blueprints/InventorySystem/DB_Items.DB_Items" "Dagger")) true (`self.ThrowSpeed`) 0.0 null))
          (bind _output_get (set `self.SlingItem` _returnvalue))
          (bind _mesh (`/Game/Blueprints/InventorySystem/BP_MasterItem.Mesh` _output_get))
          (`PrimitiveComponent.SetCollisionResponseToChannel` _mesh "ECC_GameTraceChannel2" "ECR_Ignore")
          (`PrimitiveComponent.IgnoreActorWhenMoving` _mesh self true)
          (add `/Game/Blueprints/InventorySystem/BP_MasterItem.OnProjectileImpact` _returnvalue (delegate `ProjectileDamage`)))))))

(event `ProjectileDamage`
  (params (DamagedActor :type "Actor Object Reference"))
  ;[1 0.1067 0] Attack
  ;; Sling
  (message `/Game/Blueprints/DamageSystem/BPI_StatManagement.TakeDamage` DamagedActor (make `/Game/Blueprints/DamageSystem/S_DamageInfo` 5.0 "NewEnumerator2" "NewEnumerator1" true true false false self))
  (`self.K2_DestroyActor` (`self.SlingItem`)))

(fn `AI_AttackStart`
  (params (AttackTarget :type "Actor Object Reference") (TokensNeeded :type Integer))
  (returns (Success :type Boolean))
  (bind _success (`parent.AI_AttackStart` AttackTarget TokensNeeded))
  (return _success))

(fn `AI_EquipWeapon`
  (returns (BP_EnemyBase :type "/Game/Blueprints/Enemies/BP_EnemyBase Object Reference"))
  (`self.EquipWeapon`)
  (return self))

(fn `AI_GetIdealRange`
  (returns (AttackRadius :type "Float (double-precision)") (DefendRadius :type "Float (double-precision)"))
  (return 90.0 550.0))

(fn `AI_GetPatrolRoute`
  (returns (PatrolRoute :type "/Game/Blueprints/AI/BP_PatrolRoute Object Reference"))
  (return (`self.PatrolRoute`)))

(fn `AI_SetMovementSpeed`
  (params (MovementMode :type "/Game/Blueprints/AI/Enums/E_AIMovementModes Enum" :default "NewEnumerator0"))
  (returns (Speed :type "Float (double-precision)"))
  (return (select `/Game/Blueprints/AI/Enums/E_AIMovementModes` MovementMode :`NewEnumerator1` 100.0 :`NewEnumerator2` 250.0 :`NewEnumerator3` 600.0)))

(fn `AI_UnEquipWeapon`
  (returns (BP_EnemyBase :type "/Game/Blueprints/Enemies/BP_EnemyBase Object Reference"))
  (`self.UnequipWeapon`)
  (return self))

(fn `UserConstructionScript`
  (`parent.UserConstructionScript`))